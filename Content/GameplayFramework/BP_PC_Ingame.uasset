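; In-game player controller that moves the controlled pawn and manages the local player's lobby, loading and in-game UI.
; The Enhanced Input move action is rotated by control yaw for camera-relative movement.
; Custom events create lobby, loading and in-game widgets only on the local controller, with lobby and loading also toggling the mouse cursor.
; Lobby and loading widgets have matching remove events; the in-game UI has none.
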(event `EnhancedInput|/Game/GameplayFramework/Input/IA_Move`
  (params (ActionValue :type "Vector2D Structure") (ElapsedSeconds :type "Float (double-precision)") (TriggeredSeconds :type "Float (double-precision)") (InputAction :type "InputAction Object Reference" :default "/Game/GameplayFramework/Input/IA_Move.IA_Move"))
  (bind (_returnvalue_roll _returnvalue_pitch _returnvalue_yaw) (`KismetMathLibrary.BreakRotator` (`self.GetControlRotation`)))
  ;[1 1 1] Movement
  (:`Triggered`
    (`/Engine/EditorBlueprintResources/StandardMacros.IsValid` (`self.K2_GetPawn`)
      (:`Is Valid`
        (`Pawn.AddMovementInput` (`self.K2_GetPawn`) (`KismetMathLibrary.Quat_RotateVector` (`KismetMathLibrary.Conv_RotatorToQuaternion` (`KismetMathLibrary.MakeRotator` 0.0 0.0 _returnvalue_yaw)) (`KismetMathLibrary.Conv_Vector2DToVector` ActionValue)) 1.0 false)))))

(event `self.CreateLobbyUI`
  (if (`self.IsLocalPlayerController`)
    (bind _returnvalue (`|CreateWidget` "/Game/UI/Lobby/WBP_Lobby.WBP_Lobby_C" self))
    (bind _output_get (set `self.LobbyUI` _returnvalue))
    (`UserWidget.AddToViewport` _output_get 0)
    (set `self.bShowMouseCursor` true)))

(event `self.RemoveLobbyUI`
  (`/Engine/EditorBlueprintResources/StandardMacros.IsValid` (`self.LobbyUI`)
    (:`Is Valid`
      (`Widget.RemoveFromParent` (`self.LobbyUI`))
      (set `self.LobbyUI` null))))

(event `self.CreateLoadingUI`
  (if (`self.IsLocalPlayerController`)
    (bind _returnvalue (`|CreateWidget` "/Game/UI/Lobby/WBP_LoadingScreen.WBP_LoadingScreen_C"))
    (bind _output_get (set `self.LoadingScreen` _returnvalue))
    (`UserWidget.AddToViewport` _output_get 0)
    (set `self.bShowMouseCursor` false)))

(event `self.RemoveLoadingUI`
  (`/Engine/EditorBlueprintResources/StandardMacros.IsValid` (`self.LoadingScreen`)
    (:`Is Valid`
      (`Widget.RemoveFromParent` (`self.LoadingScreen`))
      (set `self.LoadingScreen` null))))

(event `self.CreateIngameUI`
  (if (`self.IsLocalPlayerController`)
    ;[1 0.9475 0.2806] Ingame UI
    (bind _returnvalue (`|CreateWidget` "/Game/UI/IngameUI/WBP_InGameUI.WBP_InGameUI_C" self))
    (bind _output_get (set `self.InGameUI` _returnvalue))
    (`UserWidget.AddToViewport` _output_get 0)))

(fn `UserConstructionScript`)