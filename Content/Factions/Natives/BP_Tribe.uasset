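; BP_Tribe is a native faction settlement that sets itself up on the map.
; On Init it registers its population summary with the GOTA game state for totals updates and claims a random tile from the tile map.
; It then builds a first native house on that tile and seeds a starting food stockpile, printing an error if no tile was claimed.
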(event `self.Init`
  (`GOTAGameState.RegisterNativeSettlementForTotalsUpdates` (`/Game/CoreSystems/Utility/BPL_Utils.Get GOTA Game State`) (`self.PopulationSummary`))
  (`self.ClaimTile` (`TileMap.GetRandomTile` (`/Game/CoreSystems/GameplayFramework/BP_GOTAGameState.TileMap` (`/Game/CoreSystems/Utility/BPL_Utils.Get GOTA Game State`))))
  (if (`KismetArrayLibrary.Array_IsEmpty` (`self.ClaimedTiles`))
    (`KismetSystemLibrary.PrintString` "Claimed Tiles is Empty, but shouldn't be")
    (else
      ;[1 1 1] Build First House
      (`Tile.TryBuild` (`|GetArrayItem` (`self.ClaimedTiles`)) "/Game/Factions/Natives/Buildings/DA_NativeHousing.DA_NativeHousing")
      ;[1 1 1] Starting Food Stockpile
      (set `GOTAAttribute.Current` 150 (`self.Food`)))))

(fn `UserConstructionScript`
  (`parent.UserConstructionScript`))