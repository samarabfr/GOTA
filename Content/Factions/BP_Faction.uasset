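; BP_Faction is an actor representing a faction that owns a collection of settlements.
; Init takes a starting count and calls CreateSettlement that many times.
; CreateSettlement spawns a SettlementBlueprint actor at the world origin and adds it to the Settlements array, which GetSettlements returns.
; The event graph holds only disabled default events, so setup depends on Init being called.
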(fn `CreateSettlement`
  (bind _returnvalue (`|SpawnActorFromClass` (`self.SettlementBlueprint`) (`KismetMathLibrary.MakeTransform` (0.0 0.0 0.0)) "Undefined" "MultiplyWithRoot" null null))
  (`KismetArrayLibrary.Array_Add` (`self.Settlements`) _returnvalue))

(fn `GetSettlements`
  (returns (Settlements :type "Array of /Game/Factions/BP_Settlement Object Reference"))
  (return (`self.Settlements`)))

(fn `Init`
  (params (`Starting Settlement Count` :type Integer))
  (for _ (range 1 (+ `Starting Settlement Count` 1))
    (`self.CreateSettlement`)))

(fn `UserConstructionScript`)