(event `self.OnTurn`
  (params (Tile :type "Tile Object Reference"))
  (bind _claimant (`/Game/Core/World/BP_Tile.Claimant` Tile))
  (`/Engine/EditorBlueprintResources/StandardMacros.IsValid` _claimant
    (:`Is Valid`
      (`GOTAAttribute.Add` (`Settlement.Food` _claimant) (`KismetMathLibrary.FTrunc` (`self.FoodIncome`))))))

(event `self.OnClaim`
  (params (Claimant :type "Settlement Object Reference")))

(event `self.OnUnclaim`
  (params (Claimant :type "Settlement Object Reference")))

(fn `BuildPriority`
  (params (Builder :type "Settlement Object Reference"))
  (returns (ReturnValue :type Integer))
  (locals (Prio :type Integer))
  (set `local.Prio` (`KismetMathLibrary.FTrunc` (/ (- (`KismetMathLibrary.Conv_IntToDouble` (`GOTAAttribute.Current` (`Settlement.Food` (`local.Builder`)))) (`self.FoodCost`)) (`GOTAAttribute.Current` (`Settlement.Population` (`local.Builder`))))))
  (`|ExecutionSequence`
    (:`then_1`
      (return (`local.Prio`)))))

(fn `CanBuilderAfford`
  (params (Builder :type "Settlement Object Reference"))
  (returns (ReturnValue :type Boolean))
  (return (> (`KismetMathLibrary.Conv_IntToDouble` (`GOTAAttribute.Current` (`Settlement.Food` Builder))) (`self.FoodCost`))))

(fn `UserConstructionScript`)