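; Base settlement actor for factions, holding territory and replicated population, food and religion stats.
; On BeginPlay the server picks a random claim color and tile; CalculateClaiming then expands into random bordering tiles up to MaxClaims, refreshing the border after each claim.
; Setters clamp stats, religion changes split Population between colonists and natives, and RepNotifies fire change events.
; CalculateIncome and CalculateBuilding are empty, the latter left to derived classes.
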(event `self.ReceiveBeginPlay`
  (`|ExecutionSequence`
    (:`then_0`
      ;[1 1 1] Random Claim Color
      (`/Engine/EditorBlueprintResources/ActorMacros.Switch Has Authority`
        (:`Authority`
          (set `self.ClaimColor` (make `LinearColor` (`KismetMathLibrary.RandomFloat`) (`KismetMathLibrary.RandomFloat`) (`KismetMathLibrary.RandomFloat`) 1.0)))))
    (:`then_1`
      ;[1 1 1] Claim a random Tile
      (`/Engine/EditorBlueprintResources/ActorMacros.Switch Has Authority`
        (:`Authority`
          (bind _tile (`/Game/Core/TileMap/BP_TileMap.GetRandomTile` (`/Game/Core/BP_GOTAGameState.TileMap` (`/Game/Core/BPL_Utils.Get GOTA Game State`))))
          (`self.ClaimTile` _tile))))))

(event `CalculateBuilding`
  ;[1 1 1] Should be implemented by the derived Classes
)

(fn `CalculateClaiming`
  ;[1 1 1] Check for Max Claim limit
  (if (< (`KismetArrayLibrary.Array_Length` (`self.ClaimedTiles`)) (`self.MaxClaims`))
    (bind _result (`BlueprintSetLibrary.Set_ToArray` (`self.BorderingUnclaimedTiles`)))
    (`self.ClaimTile` (`KismetArrayLibrary.Array_Random` _result))))

(fn `CalculateIncome`)

(fn `ChangeColonistReligion`
  (params (Change :type Integer))
  (set `self.ColonistReligion` (`KismetMathLibrary.Min` (`KismetMathLibrary.Max` (+ Change (`self.ColonistReligion`))) (`self.Population`)))
  (set `self.NativeReligion` (- (`self.Population`) (`self.ColonistReligion`))))

(fn `ChangeNativeReligion`
  (params (Change :type Integer))
  (set `self.NativeReligion` (`KismetMathLibrary.Min` (`KismetMathLibrary.Max` (+ Change (`self.NativeReligion`))) (`self.Population`)))
  (set `self.ColonistReligion` (- (`self.Population`) (`self.NativeReligion`))))

(fn `ClaimTile`
  (params (Tile :type "/Game/Core/TileMap/BP_Tile Object Reference"))
  (`/Engine/EditorBlueprintResources/StandardMacros.IsValid` Tile
    (:`Is Valid`
      (bind _success (`/Game/Core/TileMap/BP_Tile.Claim` (`local.Tile`) self))
      (if _success
        (`KismetArrayLibrary.Array_Add` (`self.ClaimedTiles`) (`local.Tile`))
        (`self.RefreshBorderingTiles`)))))

(fn `GetColonistReligion`
  (returns (ColonistReligion :type Integer))
  (return (`self.ColonistReligion`)))

(fn `GetFood`
  (returns (Food :type Integer))
  (return (`self.Food`)))

(fn `GetMaxPopulation`
  (returns (`Max Population` :type Integer))
  (return (`self.MaxPopulation`)))

(fn `GetNativeReligion`
  (returns (NativeReligion :type Integer))
  (return (`self.NativeReligion`)))

(fn `GetPopulation`
  (returns (Population :type Integer))
  (return (`self.Population`)))

(fn `OnRep_ColonistReligion`
  (`self.OnColonistReligionChanged` (`self.ColonistReligion`)))

(fn `OnRep_Food`
  (`self.OnFoodChanged` (`self.Food`)))

(fn `OnRep_MaxPopulation`
  (`self.OnMaxPopulationChanged` (`self.MaxPopulation`)))

(fn `OnRep_NativeReligion`
  (`self.OnNativeReligionCHanged` (`self.NativeReligion`)))

(fn `OnRep_Population`
  (`self.OnPopulationChanged` (`self.Population`)))

(fn `RefreshBorderingTiles`
  (`BlueprintSetLibrary.Set_Clear` (`self.BorderingUnclaimedTiles`))
  (for _array_element (`self.ClaimedTiles`)
    (bind _neighbors (`/Game/Core/TileMap/BP_TileMap.GetNeighboringTiles` (`/Game/Core/BP_GOTAGameState.TileMap` (`/Game/Core/BPL_Utils.Get GOTA Game State`)) _array_element))
    (for _array_element_2 _neighbors
      (if (`/Game/Core/TileMap/BP_Tile.IsClaimable` _array_element_2)
        (`BlueprintSetLibrary.Set_Add` (`self.BorderingUnclaimedTiles`) _array_element_2)))))

(fn `SetFood`
  (params (`New Food` :type Integer))
  (set `self.Food` (`KismetMathLibrary.Max` `New Food`)))

(fn `SetMaxPopulation`
  (params (`New Max Population` :type Integer))
  (set `self.MaxPopulation` (`KismetMathLibrary.Max` `New Max Population`)))

(fn `SetPopulation`
  (params (`New Population` :type Integer))
  (set `self.Population` (`KismetMathLibrary.Max` `New Population`)))

(fn `UserConstructionScript`)