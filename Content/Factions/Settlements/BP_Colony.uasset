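; BP_Colony is a colonial settlement Blueprint that sets up a new colony's starting state.
; InitialStartingSetup registers its population summary with the game state for totals updates, then claims the given spawn tile, if valid and claimable, plus two random tiles.
; It builds housing, a lumbermill and an expansion building on them, seeds each with population and sets a starting food stockpile.
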(event `self.InitialStartingSetup`
  (params (SpawnTile :type "Tile Object Reference"))
  (bind _output (`|GetArrayItem` (`self.ClaimedTiles`) 2))
  (bind _output_2 (`|GetArrayItem` (`self.ClaimedTiles`)))
  (bind _output_3 (`|GetArrayItem` (`self.ClaimedTiles`) 1))
  (`GS_Ingame.RegisterColonialSettlementForTotalsUpdates` (`/Game/CoreSystems/Utility/BPL_Utils.Get GOTA Game State`) (`self.PopulationSummary`))
  (`/Engine/EditorBlueprintResources/StandardMacros.IsValid` SpawnTile
    (:`Is Valid`
      (if (`Tile.IsClaimable` SpawnTile)
        (`self.ClaimTile` SpawnTile)
        (`self.ClaimRandomTile`)
        (`self.ClaimRandomTile`)
        (`Tile.TryBuild` _output_2 "/Game/Factions/Buildings/DA_C_Housing.DA_C_Housing")
        (`Population.ChangePopulation` (`Building.Population` (`Tile.Building` _output_2)) 4)
        (`Tile.TryBuild` _output_3 "/Game/Factions/Buildings/DA_C_Lumbermill.DA_C_Lumbermill")
        (`Population.ChangePopulation` (`Building.Population` (`Tile.Building` _output_3)) 4)
        (`Tile.TryBuild` _output "/Game/Factions/Buildings/DA_C_Expansion.DA_C_Expansion")
        (`Population.ChangePopulation` (`Building.Population` (`Tile.Building` _output)) 4)
        ;[1 1 1] Starting Food Stockpile
        (set `GOTAAttribute.Current` 300 (`self.Food`))
        (else
          (`KismetSystemLibrary.PrintString` "Settlement got invalid starting Tile" true true (struct :`G` 0.66 :`B` 1.0 :`A` 1.0) 10.0 :!label _label))))
    (:`Is Not Valid`
      (goto _label))))

(fn `UserConstructionScript`
  (`parent.UserConstructionScript`))