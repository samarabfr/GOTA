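; BP_Flamey is a Guardian character whose ember effect responds to how much it moves.
; Each tick, it adds a small share of its movement speed to a Heat value and decays it slightly, so heat builds with motion and fades at rest.
; The cube of Heat feeds the FSXEmbers Niagara parameter User.Heat, making the response non-linear.
; The accumulation and decay are per frame, without delta-time scaling.
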(event `self.ReceiveTick`
  (params (DeltaSeconds :type "Float (single-precision)"))
  (`parent.ReceiveTick` DeltaSeconds)
  (bind _output_get (set `self.Heat` (* (+ (/ (`KismetMathLibrary.VSize` (`CharacterMovementComponent.GetLastUpdateVelocity` (`self.CharacterMovement`))) 100000.0) (`self.Heat`)) 0.995)))
  (`NiagaraComponent.SetNiagaraVariableFloat` (`self.FSX_Embers`) "User.Heat" (* _output_get _output_get _output_get)))

(fn `UserConstructionScript`
  (`parent.UserConstructionScript`))