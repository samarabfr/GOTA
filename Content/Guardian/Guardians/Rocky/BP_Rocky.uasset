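; Rocky guardian character, a child Blueprint that makes its Sphere component appear to roll as it moves.
; Each tick, after the parent's Tick, it scales CharacterMovement's last update velocity by RotationSpeed and applies it as world rotation to the Sphere.
; Y velocity drives roll and negated X drives pitch, with no yaw.
; The rotation step is not scaled by DeltaSeconds, so spin rate depends on frame rate.
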(event `self.ReceiveTick`
  (params (DeltaSeconds :type "Float (single-precision)"))
  (`parent.ReceiveTick` DeltaSeconds)
  (`SceneComponent.K2_AddWorldRotation` (`self.Sphere`) (`KismetMathLibrary.MakeRotator` (.y (* (`self.RotationSpeed`) (`CharacterMovementComponent.GetLastUpdateVelocity` (`self.CharacterMovement`)))) (* (.x (* (`self.RotationSpeed`) (`CharacterMovementComponent.GetLastUpdateVelocity` (`self.CharacterMovement`)))) -1.0)) false false))

(fn `UserConstructionScript`
  (`parent.UserConstructionScript`))