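; Settlement actor that holds territory on the game state's tile map, tracking its claimed tiles and claim color.
; On BeginPlay, the authority picks a random claim color, claims a random tile and calls Init.
; Each successful claim or lost claim rebuilds the set of claimable tiles bordering the territory.
; ClaimRandomNeighbor expands the territory by claiming a random tile from that set.
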(event `self.ReceiveBeginPlay`
  (`|ExecutionSequence`
    (:`then_0`
      ;[1 1 1] Random Claim Color
      (`/Engine/EditorBlueprintResources/ActorMacros.Switch Has Authority`
        (:`Authority`
          (set `self.ClaimColor` (make `LinearColor` (`KismetMathLibrary.RandomFloat`) (`KismetMathLibrary.RandomFloat`) (`KismetMathLibrary.RandomFloat`) 1.0)))))
    (:`then_1`
      ;[1 1 1] Claim a random Tile
      (`/Engine/EditorBlueprintResources/ActorMacros.Switch Has Authority`
        (:`Authority`
          (`self.ClaimTile` (`TileMap.GetRandomTile` (`/Game/Core/BP_GOTAGameState.TileMap` (`/Game/Core/BPL_Utils.Get GOTA Game State`))))
          (`self.Init`))))))

(fn `ClaimRandomNeighbor`
  (bind _result (`BlueprintSetLibrary.Set_ToArray` (`self.BorderingUnclaimedTiles`)))
  (`self.ClaimTile` (`KismetArrayLibrary.Array_Random` _result)))

(fn `ClaimTile`
  (params (Tile :type "Tile Object Reference"))
  (`/Engine/EditorBlueprintResources/StandardMacros.IsValid` Tile
    (:`Is Valid`
      (bind _success (`Tile.Claim` (`local.Tile`) self))
      (if _success
        (`KismetArrayLibrary.Array_Add` (`self.ClaimedTiles`) (`local.Tile`))
        (`self.RefreshBorderingTiles`)))))

(fn `LostClaim`
  (params (Tile :type "Tile Object Reference"))
  (`/Engine/EditorBlueprintResources/StandardMacros.IsValid` Tile
    (:`Is Valid`
      (`KismetArrayLibrary.Array_RemoveItem` (`self.ClaimedTiles`) (`local.Tile`))
      (`self.RefreshBorderingTiles`))))

(fn `RefreshBorderingTiles`
  (`BlueprintSetLibrary.Set_Clear` (`self.BorderingUnclaimedTiles`))
  (for _array_element (`self.ClaimedTiles`)
    (for _array_element_2 (`TileMap.GetNeighboringTiles` (`/Game/Core/BP_GOTAGameState.TileMap` (`/Game/Core/BPL_Utils.Get GOTA Game State`)) _array_element)
      (if (`/Game/Core/TileMap/BP_Tile.IsClaimable` _array_element_2)
        (`BlueprintSetLibrary.Set_Add` (`self.BorderingUnclaimedTiles`) _array_element_2)))))

(fn `UserConstructionScript`)