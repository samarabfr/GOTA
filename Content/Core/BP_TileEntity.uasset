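; BP_TileEntity is a randomly colored actor that wanders the game state's TileMap, heading from a random start tile toward random targets.
; Each Move call re-queries the path, updates a spawned BP_Path visual and steps up to Speed tiles, picking a new target when the path empties.
; Steps toggle tile walkability to mark occupancy and attach the actor to its tile, re-pinning the target marker mesh.
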(event `self.ReceiveBeginPlay`
  (bind _newparam (`/Game/Core/BPL_Utils.Get GOTA Game State`))
  (`/Engine/EditorBlueprintResources/StandardMacros.IsValid` _newparam
    (:`Is Valid`
      (`self.SetTileMap` (`/Game/Core/BP_GOTAGameState.TileMap` _newparam))
      (`self.SetSpeed` 1)
      ;[1 0.246 0.2614] Visual Path
      (bind _returnvalue (`|SpawnActorFromClass` "/Game/Core/BP_Path.BP_Path_C" (`KismetMathLibrary.MakeTransform` (0.0 0.0 0.0)) "Undefined" "MultiplyWithRoot" null null))
      (set `self.VisualPath` _returnvalue)
      ;[1 0.4646 0.9367] Random Color
      (set `self.Linear Color` (make `LinearColor` (`KismetMathLibrary.RandomFloat`) (`KismetMathLibrary.RandomFloat`) (`KismetMathLibrary.RandomFloat`) (`KismetMathLibrary.RandomFloat`)))
      (bind _returnvalue_2 (`PrimitiveComponent.CreateDynamicMaterialInstance` (`self.EntityMesh`) 0 null "None"))
      (`MaterialInstanceDynamic.SetVectorParameterValue` _returnvalue_2 "Color" (`self.Linear Color`))
      (bind _returnvalue_3 (`PrimitiveComponent.CreateDynamicMaterialInstance` (`self.MoveTargetMesh`) 0 null "None"))
      (`MaterialInstanceDynamic.SetVectorParameterValue` _returnvalue_3 "Color" (`self.Linear Color`)))))

(event `MoveTargetChanged`
  (params (MoveTarget :type "/Game/Core/TileMap/BP_Tile Object Reference"))
  (`/Engine/EditorBlueprintResources/StandardMacros.IsValid` (`self.MoveTarget`) :!label _label
    (:`Is Valid`
      (`SceneComponent.K2_SetWorldLocation` (`self.MoveTargetMesh`) (`self.K2_GetActorLocation` (`self.MoveTarget`)) false false))))

(event `CurrentTileChanged`
  (params (CurrentTarget :type "/Game/Core/TileMap/BP_Tile Object Reference"))
  (`self.K2_AttachToActor` CurrentTarget "None" "KeepRelative" "KeepRelative" "KeepRelative")
  (goto _label))

(event `PathChanged`
  (params (Path :type "Array of /Game/Core/TileMap/BP_Tile Object Reference"))
  (`/Game/Core/BP_Path.SetPathPoints` (`self.VisualPath`) Path))

(event `TargetReached`
  (bind _tilemap (`self.TileMap`))
  (`/Engine/EditorBlueprintResources/StandardMacros.IsValid` _tilemap :!label _label_2
    (:`Is Valid`
      (bind _tile (`/Game/Core/TileMap/BP_TileMap.GetRandomTile` _tilemap))
      (bind _output_get (set `self.MoveTarget` _tile))
      (`self.MoveTargetChanged` _output_get))))

(event `TargetUnreachable`
  (goto _label_2))

(event `TileMapChanged`
  (params (TileMap :type "/Game/Core/TileMap/BP_TileMap Object Reference"))
  (`/Engine/EditorBlueprintResources/StandardMacros.IsValid` TileMap
    (:`Is Valid`
      (bind _tile (`/Game/Core/TileMap/BP_TileMap.GetRandomTile` (`self.TileMap`)))
      (bind _output_get (set `self.CurrentTile` _tile))
      (`self.CurrentTileChanged` _output_get)
      (bind _tile_2 (`/Game/Core/TileMap/BP_TileMap.GetRandomTile` (`self.TileMap`)))
      (bind _output_get_2 (set `self.MoveTarget` _tile_2))
      (`self.MoveTargetChanged` _output_get_2))))

(fn `Move`
  (bind _tilemap (`self.TileMap`))
  (bind _path (`self.Path`))
  (bind _output (`|GetArrayItem` _path (`KismetArrayLibrary.Array_LastIndex` _path)))
  ;[0.2747 0.2543 1] Get New Path
  (`/Engine/EditorBlueprintResources/StandardMacros.IsValid` _tilemap
    (:`Is Valid`
      (bind _output_get (set `self.Path` (`/Game/Core/TileMap/BP_TileMap.GetPath` _tilemap (`self.CurrentTile`) (`self.MoveTarget`))))
      (`self.PathChanged` _output_get)
      ;[0.08541 1 0.434] Move step by step
      (for _ (range 1 (+ (`self.Speed`) 1))
        (if (`KismetArrayLibrary.Array_IsNotEmpty` (`self.Path`))
          (`self.MoveTo` _output)
          (`KismetArrayLibrary.Array_RemoveItem` (`self.Path`) _output)))
      ;[1 0.5506 0.1137] Finished the path
      (if (`KismetArrayLibrary.Array_IsEmpty` (`self.Path`))
        (if (== (`self.CurrentTile`) (`self.MoveTarget`))
          (`self.TargetReached`)
          (else
            (`self.TargetUnreachable`)))))
    (:`Is Not Valid`
      (`KismetSystemLibrary.PrintString` "TileMap not found in TileEntity"))))

(fn `MoveTo`
  (params (Tile :type "/Game/Core/TileMap/BP_Tile Object Reference"))
  (bind _currenttile (`self.CurrentTile`))
  (`/Engine/EditorBlueprintResources/StandardMacros.IsValid` Tile
    (:`Is Valid`
      (`/Engine/EditorBlueprintResources/StandardMacros.IsValid` _currenttile
        (:`Is Valid`
          (set `/Game/Core/TileMap/BP_Tile.IsWalkable` true _currenttile))
        (:`Is Not Valid`
          _))
      (bind _output_get (set `self.CurrentTile` (`local.Tile`)))
      (set `/Game/Core/TileMap/BP_Tile.IsWalkable` false _output_get)
      (`self.CurrentTileChanged` _output_get))))

(fn `SetMoveTarget`
  (params (MoveTarget :type "/Game/Core/TileMap/BP_Tile Object Reference"))
  (bind _output_get (set `self.MoveTarget` MoveTarget))
  (`self.MoveTargetChanged` _output_get))

(fn `SetSpeed`
  (params (Speed :type Integer))
  (set `self.Speed` (`KismetMathLibrary.Max` Speed)))

(fn `SetTileMap`
  (params (TileMap :type "/Game/Core/TileMap/BP_TileMap Object Reference"))
  (bind _output_get (set `self.TileMap` TileMap))
  (`self.TileMapChanged` _output_get))

(fn `UserConstructionScript`)