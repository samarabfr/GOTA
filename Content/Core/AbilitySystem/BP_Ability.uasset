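; Base ability Blueprint that derived abilities extend to target a tile and act on it when activated.
; Activate ends targeting, then calls the overridable OnActivate if the tile is valid.
; Helper events construct effect objects from a class and apply them to tiles or settlements.
; Targeting toggles locally for immediate response, syncs via server RPC, and OnRep fires start/stop hooks elsewhere without re-triggering the initiating client.
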(event `Effect On Tile`
  (params (`Target Tile` :type "/Game/Core/World/Tile/BP_Tile Object Reference") (`Effect Class` :type "/Game/Core/AbilitySystem/BP_GameplayEffect Class Reference"))
  ;[1 1 1] Valid Checks
  (`/Engine/EditorBlueprintResources/StandardMacros.IsValid` `Target Tile`
    (:`Is Valid`
      (if (`KismetSystemLibrary.IsValidClass` `Effect Class`)
        ;[1 1 1] Create Ability Effect Instance and apply its effect on Target
        (bind _returnvalue (`|GenericCreateObject` `Effect Class`))
        (`/Game/Core/AbilitySystem/BP_GameplayEffect.ApplyOnTile` _returnvalue `Target Tile`)))))

(event `Effect On Settlement`
  (params (Settlement :type "Settlement Object Reference") (`Effect Class` :type "/Game/Core/AbilitySystem/BP_GameplayEffect Class Reference"))
  ;[1 1 1] Valid Checks
  (`/Engine/EditorBlueprintResources/StandardMacros.IsValid` Settlement
    (:`Is Valid`
      (if (`KismetSystemLibrary.IsValidClass` `Effect Class`)
        ;[1 1 1] Create Ability Effect Instance and apply its effect on Target
        (bind _returnvalue (`|GenericCreateObject` `Effect Class`))
        (`/Game/Core/AbilitySystem/BP_GameplayEffect.ApplyOnSettlement` _returnvalue Settlement)))))

(event `On Activate`
  (params (`Target Tile` :type "/Game/Core/World/Tile/BP_Tile Object Reference"))
  ;[1 1 1] This should not be implemented here. It should be implemented in derived Ability Blueprint Classes to set the behaviour on Ability Activation
)

(event `On Start Targeting`
  ;[1 1 1] Abilties should overwrite this to set the behaviour they want to happen when this ability will start/stop targeting
)

(event `On Stop Targeting`
  ;[1 1 1] Abilties should overwrite this to set the behaviour they want to happen when this ability will start/stop targeting
)

(event `SetNetTargetingOnServer`
  (params (`New Targeting` :type Boolean))
  ;[1 1 1] This Server RPC is needed because we can't set the bool on client and expect it to replicate. Don't call this anywhere else than inside SetTargeting
  (set `self.NetIsTargeting` `New Targeting`))

(fn `Activate`
  (params (`Target Tile` :type "/Game/Core/World/Tile/BP_Tile Object Reference"))
  ;[1 1 1] This only checks if the Target Tile is Valid and calls the OnActivate Event that should be implemented by every Ability. Im not sure if we should have more parameter to target Settlemens, Units, GUardians here or if every Ability should do its own valid checks on the Tile
  (`self.SetTargeting` false)
  (`/Engine/EditorBlueprintResources/StandardMacros.IsValid` `Target Tile`
    (:`Is Valid`
      (`self.On Activate` `Target Tile`))
    (:`Is Not Valid`
      (`KismetSystemLibrary.PrintString` "Ability Canceled, no Tile selected"))))

(fn `GetIsTargeting`
  (returns (IsTargeting :type Boolean))
  (return (`self.IsTargeting`)))

(fn `OnRep_NetIsTargeting`
  ;[1 1 1] This will be called on the Server and every client when NetIsTargeting changes. It is different than C++ OnRep in that regard.
  ;[1 1 1] Check if the local IsTargeting is already stop the client that already set it by himself to trigger StartTargeting again
  (if (not (== (`self.IsTargeting`) (`self.NetIsTargeting`)))
    ;[1 1 1] Yes this is redundant with SetTargeting. But if i call SetTargeting i get into an infinite loop, i think... idk what im doing
    (bind _output_get (set `self.IsTargeting` (`self.NetIsTargeting`)))
    (if _output_get
      (`self.On Start Targeting`)
      (else
        (`self.On Stop Targeting`)))))

(fn `SetTargeting`
  (params (`New Is Targeting` :type Boolean))
  ;[1 1 1] Check if the value stayed the same
  (if (not (== `New Is Targeting` (`self.IsTargeting`)))
    ;[1 1 1] Set it directly on own Client to have immediate change
    (bind _output_get (set `self.IsTargeting` `New Is Targeting`))
    (if _output_get
      (`self.On Start Targeting`)
      (else
        (`self.On Stop Targeting`)))
    ;[1 1 1] Tell the server to change it for him and everyone else
    (`self.SetNetTargetingOnServer` `New Is Targeting`)))

(fn `UserConstructionScript`)