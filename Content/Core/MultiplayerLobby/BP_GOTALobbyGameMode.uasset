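; BP_GOTALobbyGameMode is the game mode for the multiplayer lobby, registering connecting players into one of four lobby slots.
; On PostLogin it prints a connection message, then stores the new player's PlayerState in the first slot without a valid one on BP_GOTALobbyGameState.
; A player joining when all four slots are valid gets no slot.
; The logout event is empty, so this game mode does not clear slots.
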(event `self.K2_PostLogin`
  (params (NewPlayer :type "PlayerController Object Reference"))
  (bind _playerstate (`Controller.PlayerState` NewPlayer))
  ;[1 1 1] Log output
  (`KismetSystemLibrary.PrintString` (`KismetStringLibrary.Concat_StrStr` (`KismetSystemLibrary.GetDisplayName` NewPlayer) " connected!"))
  (bind _asbp_gotalobby_game_state (cast `/Game/Core/MultiplayerLobby/BP_GOTALobbyGameState` (`GameplayStatics.GetGameState`)))
  (bind _lobbyplayer1 (`GOTALobbyGameState.LobbyPlayer1` _asbp_gotalobby_game_state))
  (`/Engine/EditorBlueprintResources/StandardMacros.IsValid` (`LobbyPlayer.PlayerState` _lobbyplayer1)
    (:`Is Valid`
      (bind _lobbyplayer2 (`GOTALobbyGameState.LobbyPlayer2` _asbp_gotalobby_game_state))
      (`/Engine/EditorBlueprintResources/StandardMacros.IsValid` (`LobbyPlayer.PlayerState` _lobbyplayer2)
        (:`Is Valid`
          (bind _lobbyplayer3 (`GOTALobbyGameState.LobbyPlayer3` _asbp_gotalobby_game_state))
          (`/Engine/EditorBlueprintResources/StandardMacros.IsValid` (`LobbyPlayer.PlayerState` _lobbyplayer3)
            (:`Is Valid`
              (bind _lobbyplayer4 (`GOTALobbyGameState.LobbyPlayer4` _asbp_gotalobby_game_state))
              (`/Engine/EditorBlueprintResources/StandardMacros.IsValid` (`LobbyPlayer.PlayerState` _lobbyplayer4)
                (:`Is Not Valid`
                  (set `LobbyPlayer.PlayerState` _playerstate _lobbyplayer4))))
            (:`Is Not Valid`
              (set `LobbyPlayer.PlayerState` _playerstate _lobbyplayer3))))
        (:`Is Not Valid`
          (set `LobbyPlayer.PlayerState` _playerstate _lobbyplayer2))))
    (:`Is Not Valid`
      (set `LobbyPlayer.PlayerState` _playerstate _lobbyplayer1))))

(event `self.K2_OnLogout`
  (params (ExitingController :type "Controller Object Reference")))

(fn `UserConstructionScript`)