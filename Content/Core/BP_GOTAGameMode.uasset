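; Game mode for GOTA that runs timed turns on the server and provides setup events for the match.
; Setup spawns a circular island tile map, Colonist and Native factions and four Guardians, which player controllers possess by index.
; On Tick, an expired turn timer on the GameState triggers a synchronous calculation: settlements update, then tile entities move.
; Timer ticking pauses during calculation, with start/end notifications sent through the GameState and the duration printed.
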(event `self.ReceiveTick`
  (params (DeltaSeconds :type "Float (single-precision)"))
  (`/Engine/EditorBlueprintResources/ActorMacros.Switch Has Authority`
    (:`Authority`
      (`/Engine/EditorBlueprintResources/StandardMacros.IsValid` (`self.Game State`)
        (:`Is Valid`
          (if (`GOTAGameState.ShouldTickTurnTime` (`self.Game State`))
            ;[1 1 1] Check if Turn is finished
            (if (>= (`/Game/Core/BP_GOTAGameState.ElapsedTurnTime` (`self.Game State`)) (`/Game/Core/BP_GOTAGameState.MaxTurnTime` (`self.Game State`)))
              (`GOTAGameState.MulticastSetElapsedTurnTime` (`self.Game State`) 0.0)
              (`self.NotAsyncTurnCalc`))))))))

(event `NotAsyncTurnCalc`
  (`self.OnTurnCalculationStart`)
  (`self.CalculateTurn`)
  (`self.OnTurnCalculationEnd`))

(event `OnTurnCalculationStart`
  (set `GOTAGameState.ShouldTickTurnTime` false (`self.Game State`))
  (set `GOTAGameState.IsCalculatingTurn` true (`self.Game State`))
  (set `self.TurnCalculationTime` (`KismetMathLibrary.Now`))
  (`GOTAGameState.CallCalculationStart` (`self.Game State`)))

(event `OnTurnCalculationEnd`
  (bind (_days _hours _minutes _seconds _fractionnano) (`KismetMathLibrary.BreakTimespan2` (- (`KismetMathLibrary.Now`) (`self.TurnCalculationTime`))))
  (set `GOTAGameState.ShouldTickTurnTime` true (`self.Game State`))
  (set `GOTAGameState.IsCalculatingTurn` false (`self.Game State`))
  (`KismetSystemLibrary.PrintString` (`KismetStringLibrary.Concat_StrStr` "Turn calc time (ms): " (`KismetStringLibrary.Conv_IntToString` (+ (* _seconds 1000) (/ _fractionnano 1000000)))))
  (`GOTAGameState.CallCalculationEnd` (`self.Game State`)))

(event `self.Init`
  ;[1 1 1] Game State
  (set `self.Game State` (`/Game/Core/BPL_Utils.Get GOTA Game State`)))

(event `self.CreateMap`
  ;[1 1 1] creating the TileMap
  (bind _returnvalue (`|SpawnActorFromClass` "/Game/Core/World/BP_TileMap.BP_TileMap_C" (`KismetMathLibrary.MakeTransform` (0.0 0.0 0.0)) "Undefined" "MultiplyWithRoot" null null))
  (bind _output_get (set `GOTAGameState.TileMap` _returnvalue (`self.Game State`)))
  (`TileMap.Init` _output_get (`GOTAGameInstance.IslandRadius` (`/Game/Core/BPL_Utils.Get GOTA Game Instance`)))
  (`/Game/Core/World/BP_TileMap.GenerateCircle` _output_get (`self.Island Radius`)))

(event `self.CreateFactions`
  ;[0.3542 0.3542 0.3542] Factions
  ;;[1 1 1] Natives
  (bind _returnvalue (`|SpawnActorFromClass` "/Game/Factions/Colonists/BP_Colonists.BP_Colonists_C" (`KismetMathLibrary.MakeTransform` (0.0 0.0 0.0)) "Undefined" "MultiplyWithRoot" null null))
  (`Faction.Init` _returnvalue (`self.InvaderStartingSettlementCount`))
  (`GOTAGameState.AddFaction` (`self.Game State`) _returnvalue)
  ;;[1 1 1] Invader
  (bind _returnvalue_2 (`|SpawnActorFromClass` "/Game/Factions/Natives/BP_Natives.BP_Natives_C" (`KismetMathLibrary.MakeTransform` (0.0 0.0 0.0)) "Undefined" "MultiplyWithRoot" null null))
  (`Faction.Init` _returnvalue_2 (`self.NativeStartingSettlementCount`))
  (`GOTAGameState.AddFaction` (`self.Game State`) _returnvalue_2))

(event `self.CreateGuardians`
  (bind _returnvalue (`|SpawnActorFromClass` "/Game/Guardians/Flamey/BP_Flameboy.BP_Flameboy_C" (`KismetMathLibrary.MakeTransform` (0.0 0.0 1000.0)) "AdjustIfPossibleButAlwaysSpawn" "MultiplyWithRoot" null null))
  (`KismetArrayLibrary.Array_Add` (`GOTAGameState.Guardians` (`self.Game State`)) _returnvalue)
  (bind _returnvalue_2 (`|SpawnActorFromClass` "/Game/Guardians/Rocky/BP_Rocky.BP_Rocky_C" (`KismetMathLibrary.MakeTransform` (0.0 0.0 1200.0)) "AdjustIfPossibleButAlwaysSpawn" "MultiplyWithRoot" null null))
  (`KismetArrayLibrary.Array_Add` (`GOTAGameState.Guardians` (`self.Game State`)) _returnvalue_2)
  (bind _returnvalue_3 (`|SpawnActorFromClass` "/Game/Guardians/Planty/BP_Planty.BP_Planty_C" (`KismetMathLibrary.MakeTransform` (0.0 0.0 1400.0)) "AdjustIfPossibleButAlwaysSpawn" "MultiplyWithRoot" null null))
  (`KismetArrayLibrary.Array_Add` (`GOTAGameState.Guardians` (`self.Game State`)) _returnvalue_3)
  (bind _returnvalue_4 (`|SpawnActorFromClass` "/Game/Guardians/Splashy/BP_Splashy.BP_Splashy_C" (`KismetMathLibrary.MakeTransform` (0.0 0.0 1600.0)) "AdjustIfPossibleButAlwaysSpawn" "MultiplyWithRoot" null null))
  (`KismetArrayLibrary.Array_Add` (`GOTAGameState.Guardians` (`self.Game State`)) _returnvalue_4))

(event `self.InitialPlayerControllerPossession`
  (for _index (range (`GameplayStatics.GetNumPlayerControllers`))
    (bind _asbp_gotaplayer_controller (cast `/Game/Core/BP_GOTAPlayerController` (`GameplayStatics.GetPlayerController` _index))
      (:`then`
        (bind _asbp_guardian (cast `/Game/Core/World/BP_Guardian` (`|GetArrayItem` (`GOTAGameState.Guardians` (`self.Game State`)) _index)))
        (`/Game/Core/BP_GOTAPlayerController.Possess Guardian` _asbp_gotaplayer_controller _asbp_guardian))
      (:`CastFailed`
        (`KismetSystemLibrary.PrintString` "Using the wrong Player Controller")))))

(event `self.StartGame`
  (set `GOTAGameState.ShouldTickTurnTime` true (`self.Game State`)))

(fn `CalculateTurn`
  (`|ExecutionSequence`
    (:`then_1`
      ;[1 1 1] Settlements Claims
      (for _array_element (`GOTAGameState.Factions` (`self.Game State`))
        (for _array_element_2 (`Faction.Settlements` _array_element)
          (`/Game/Core/World/BP_Settlement.CalculateTurn` _array_element_2))))
    (:`then_3`
      ;[1 1 1] Units bewegn
      (for _array_element_3 (`GOTAGameState.TileEntities` (`self.Game State`))
        (`TileEntity.Move` _array_element_3)))))

(fn `UserConstructionScript`)