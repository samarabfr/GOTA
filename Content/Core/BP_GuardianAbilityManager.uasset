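; Guardian ability manager that spawns the player's ability actors and handles targeting and activating them on map tiles.
; Setting MouseUtils learns four fixed abilities, each spawned as an owned actor, stored in an array and attached to the mouse's tile position.
; Triggering by index starts targeting and cancels any other targeting ability, or activates an already-targeting one on the hovered tile.
; A separate trigger activates the current targeting ability.
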(event `LearnNewAbility`
  (params (AbilityClass :type "/Game/Core/BP_Ability Class Reference"))
  (bind _returnvalue (`|SpawnActorFromClass` AbilityClass (`KismetMathLibrary.MakeTransform` (0.0 0.0 0.0)) "Undefined" "MultiplyWithRoot" null null))
  (`Actor.SetOwner` _returnvalue (`self.GetOwner`))
  (`KismetArrayLibrary.Array_Add` (`self.Abilities`) _returnvalue)
  ;[1 1 1] check mouse utils because we need to attach the ability to it
  (`/Engine/EditorBlueprintResources/StandardMacros.IsValid` (`self.MouseUtils`)
    (:`Is Valid`
      (`/Game/Core/BP_MouseUtils.AttachToTilePosition` (`self.MouseUtils`) _returnvalue))))

(fn `SetMouseUtils`
  (params (`Mouse Utils` :type "/Game/Core/BP_MouseUtils Object Reference"))
  (set `self.MouseUtils` `Mouse Utils`)
  (`self.LearnNewAbility` "/Game/Abilities/CityOfFlames/AB_CityOfFlames.AB_CityOfFlames_C")
  (`self.LearnNewAbility` "/Game/Abilities/Earthquake/AB_Earthquake.AB_Earthquake_C")
  (`self.LearnNewAbility` "/Game/Abilities/FertileLands/AB_FertileLands.AB_FertileLands_C")
  (`self.LearnNewAbility` "/Game/Abilities/GrowNature/AB_GrowNature.AB_GrowNature_C"))

(fn `SetPlayerController`
  (params (PlayerController :type "/Game/Core/BP_GOTAPlayerController Object Reference"))
  (set `self.PlayerController` PlayerController))

(fn `TriggerAbilityByIndex`
  (params (Index :type Integer))
  (locals (InputAbility :type "/Game/Core/BP_Ability Object Reference"))
  ;[1 1 1] Get Input Ability from Array and check if it is Valid
  (if (`KismetArrayLibrary.Array_IsValidIndex` (`self.Abilities`) Index)
    (bind _output_get (set `local.InputAbility` (`|GetArrayItem` (`self.Abilities`) (`local.Index`))))
    (`/Engine/EditorBlueprintResources/StandardMacros.IsValid` _output_get
      (:`Is Valid`
        ;[1 1 1] Check if Input Ability is Targeting rn
        (if (`/Game/Core/BP_Ability.GetIsTargeting` (`local.InputAbility`))
          ;[1 1 1] Activate Input Ability
          (`/Game/Core/BP_Ability.Activate` (`local.InputAbility`) (`/Game/Core/BP_MouseUtils.HoverTile` (`self.MouseUtils`)))
          (else
            ;[1 1 1] Check if Input Ability is the same as the Current Targeting Ability
            (if (not (== (`local.InputAbility`) (`self.CurrentTargetingAbility`)))
              ;[1 1 1] Cancel Current Target Ability if another Ability starts targeting
              (`/Engine/EditorBlueprintResources/StandardMacros.IsValid` (`self.CurrentTargetingAbility`)
                (:`Is Valid`
                  (`/Game/Core/BP_Ability.SetTargeting` (`self.CurrentTargetingAbility`) false))
                (:`Is Not Valid`
                  _)))
            ;[1 1 1] Set Targeting on Input Ability
            (`/Game/Core/BP_Ability.SetTargeting` (`local.InputAbility`) true)
            (set `self.CurrentTargetingAbility` (`local.InputAbility`)))))
      (:`Is Not Valid`
        (`KismetSystemLibrary.PrintString` "GAM: Invalid Ability")))
    (else
      (`KismetSystemLibrary.PrintString` "GAM: Invalid Index"))))

(fn `TriggerCurrentTargetingAbility`
  (`/Engine/EditorBlueprintResources/StandardMacros.IsValid` (`self.CurrentTargetingAbility`)
    (:`Is Valid`
      (if (`/Game/Core/BP_Ability.GetIsTargeting` (`self.CurrentTargetingAbility`))
        ;[1 1 1] Activate Current Ability
        (`/Game/Core/BP_Ability.Activate` (`self.CurrentTargetingAbility`) (`/Game/Core/BP_MouseUtils.HoverTile` (`self.MouseUtils`)))))))