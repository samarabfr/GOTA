(fn `Build`
  (params (BuildingClass :type "Building Class Reference"))
  (returns (Success :type Boolean))
  ;[1 1 1] Can only be called by Server
  ;[1 1 1] Already a Building on this Tile
  (`/Engine/EditorBlueprintResources/StandardMacros.IsValid` (`self.Building`)
    (:`Is Valid`
      (return false))
    (:`Is Not Valid`
      (`|ExecutionSequence`
        (:`then_0`
          ;[1 1 1] Create Building Object
          (bind _returnvalue (`|GenericCreateObject` (`local.BuildingClass`)))
          (bind _output_get (set `self.Building` _returnvalue))
          ;[1 1 1] Trigger OnBuild
          (`Building.OnBuild` _output_get self))
        (:`then_1`
          ;[1 1 1] If claimed, trigger OnClaim
          (`/Engine/EditorBlueprintResources/StandardMacros.IsValid` (`self.Claimant`)
            (:`Is Valid`
              (`Building.OnClaim` (`self.Building`) (`self.Claimant`)))))
        (:`then_2`
          ;[1 1 1] Set Graphics
          (`StaticMeshComponent.SetStaticMesh` (`self.BuildingMesh`) (`Building.Mesh` (`self.Building`))))
        (:`then_3`
          (return true))))))

(fn `Claim`
  (params (PotentialClaimant :type "Settlement Object Reference"))
  (returns (Success :type Boolean))
  ;[1 1 1] Can only be called by Server
  ;[1 1 1] not claimable
  (if (`self.IsClaimable`)
    (`|ExecutionSequence`
      (:`then_0`
        ;[1 1 1] Set instance variables
        (set `self.Claimant` (`local.PotentialClaimant`))
        (set `self.IsClaimable` false))
      (:`then_1`
        ;[1 0.452 0.332] Trigger Building Claim Effect if there is a Building on the Tile
        (`/Engine/EditorBlueprintResources/StandardMacros.IsValid` (`self.Building`)
          (:`Is Valid`
            (`Building.OnClaim` (`self.Building`) (`self.Claimant`)))))
      (:`then_2`
        (return true)))
    (else
      (return false))))

(fn `ClaimantChanged`
  (`/Engine/EditorBlueprintResources/StandardMacros.IsValid` (`self.Claimant`)
    (:`Is Valid`
      ;[1 1 1] Tile is now claimed
      (`SceneComponent.SetVisibility` (`self.ClaimMesh`) true false)
      (`MeshComponent.SetVectorParameterValueOnMaterials` (`self.ClaimMesh`) "Color" (`KismetMathLibrary.Conv_LinearColorToVector` (`Settlement.ClaimColor` (`self.Claimant`)))))
    (:`Is Not Valid`
      ;[1 1 1] Tile is not claimed anymore
      (`SceneComponent.SetVisibility` (`self.ClaimMesh`) false false))))

(fn `Unbuild`
  ;[1 1 1] Can only be called by Server
  ;[1 1 1] Has no Building
  (`/Engine/EditorBlueprintResources/StandardMacros.IsValid` (`self.Building`)
    (:`Is Valid`
      (`|ExecutionSequence`
        (:`then_0`
          ;[1 1 1] If claimed, trigger OnUnclaim
          (`/Engine/EditorBlueprintResources/StandardMacros.IsValid` (`self.Claimant`)
            (:`Is Valid`
              (`Building.OnUnclaim` (`self.Building`) (`self.Claimant`)))))
        (:`then_1`
          ;[1 1 1] Trigger OnUnbuild of the Building
          (`Building.OnUnbuild` (`self.Building`) self))
        (:`then_2`
          ;[1 1 1] Set Graphics
          (`StaticMeshComponent.SetStaticMesh` (`self.BuildingMesh`) null))
        (:`then_3`
          ;[1 1 1] Remove Building reference
          (set `self.Building` null))))
    (:`Is Not Valid`
      (return))))

(fn `Unclaim`
  ;[1 1 1] Can only be called by Server
  ;[1 1 1] Has Claimant
  (`/Engine/EditorBlueprintResources/StandardMacros.IsValid` (`self.Claimant`)
    (:`Is Valid`
      (`|ExecutionSequence`
        (:`then_0`
          ;[1 0.452 0.332] Trigger Building Unclaim Effect if there is a Building on the Tile
          (`/Engine/EditorBlueprintResources/StandardMacros.IsValid` (`self.Building`)
            (:`Is Valid`
              (`Building.OnUnclaim` (`self.Building`) (`self.Claimant`)))))
        (:`then_1`
          ;[1 1 1] Tell Settlement that it lost this claim
          (`Settlement.LostClaim` (`self.Claimant`) self))
        (:`then_2`
          ;[1 1 1] Set instance variables
          (set `self.Claimant` null)
          (set `self.IsClaimable` true))))
    (:`Is Not Valid`
      (return))))

(fn `UserConstructionScript`)