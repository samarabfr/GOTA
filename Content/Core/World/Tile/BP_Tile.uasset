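; Hex world tile that settlements can claim and that holds a single building.
; The server randomizes layout, mesh and rotation; the replicated layout's OnRep waits for the attached BP_TileContent, spawned in BeginPlay, to initialize it.
; Server-only Claim and Build functions, with their inverses, keep claimant and replicated Building object notified of each other.
; It also tints the claim mesh, varies material noise offsets and forwards Guardian range events to its content.
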(event `self.ReceiveBeginPlay`
  (bind _tilelayouts (`self.TileLayouts`))
  (bind _sm_hexagon (`self.SM_Hexagon`))
  (`|ExecutionSequence`
    (:`then_0`
      (`/Engine/EditorBlueprintResources/ActorMacros.Switch Has Authority`
        (:`Authority`
          (bind _outrownames (`DataTableFunctionLibrary.GetDataTableRowNames` _tilelayouts))
          (bind _returnvalue (`|GetDataTableRow` _tilelayouts (`KismetArrayLibrary.Array_Random` _outrownames))
            (:`then`
              (bind (_tileid _mesh _riverconnections _spawnpointlayouts) (break `/Game/Core/World/Tile/F_TileLayout` _returnvalue))
              (if (not (`KismetArrayLibrary.Array_IsEmpty` _spawnpointlayouts))
                (set `self.SpawnPointLayout` (`KismetArrayLibrary.Array_Random` _spawnpointlayouts))
                (`StaticMeshComponent.SetStaticMesh` (`self.SM_Hexagon`) _mesh)
                (`self.K2_SetActorRotation` self (`KismetMathLibrary.MakeRotator` 0.0 0.0 (`KismetMathLibrary.Conv_IntToDouble` (* (`KismetMathLibrary.RandomIntegerInRange` 0 5) 60))) false)))))))
    (:`then_1`
      (bind _returnvalue_2 (`|SpawnActorFromClass` "/Game/Core/World/Tile/BP_TileContent.BP_TileContent_C" (`KismetMathLibrary.MakeTransform` (0.0 0.0 0.0)) "Undefined" "MultiplyWithRoot" null null))
      (`self.K2_AttachToActor` _returnvalue_2 self "None" "SnapToTarget" "SnapToTarget" "SnapToTarget" true)
      (set `self.TileContent` _returnvalue_2)
      ;[1 1 1] Set random offsets for material for noise variation between tiles
      (`MeshComponent.SetScalarParameterValueOnMaterials` _sm_hexagon "Offset U" (`KismetMathLibrary.RandomFloatInRange` 0.0 0.2))
      (`MeshComponent.SetScalarParameterValueOnMaterials` _sm_hexagon "Offset V" (`KismetMathLibrary.RandomFloatInRange` 0.0 0.2)))))

(event `OnRep_SpawnPointLayout`
  ;[1 1 1] Wait For TileContent to exist
  (`/Engine/EditorBlueprintResources/StandardMacros.IsValid` (`self.TileContent`) :!label _label
    (:`Is Valid`
      (`/Game/Core/World/Tile/BP_TileContent.Init` (`self.TileContent`) (`self.SpawnPointLayout`)))
    (:`Is Not Valid`
      (`KismetSystemLibrary.Delay` 0.2)
      (goto _label))))

(event `self.OnEnteringActiveRangeOfGuardian`
  (`/Game/Core/World/Tile/BP_TileContent.EnteringActiveRangeOfPlayer` (`self.TileContent`)))

(event `self.OnLeavingActiveRangeOfGuardian`
  (`/Game/Core/World/Tile/BP_TileContent.LeavingActiveRangeOfPlayer` (`self.TileContent`)))

(fn `Build`
  (params (BuildingClass :type "Building Class Reference"))
  (returns (Success :type Boolean))
  ;[1 1 1] Can only be called by Server
  ;[1 1 1] Already a Building on this Tile
  (`/Engine/EditorBlueprintResources/StandardMacros.IsValid` (`self.Building`)
    (:`Is Valid`
      (return false))
    (:`Is Not Valid`
      (`|ExecutionSequence`
        (:`then_0`
          ;[1 1 1] Create Building Object
          (bind _returnvalue (`|GenericCreateObject` (`local.BuildingClass`)))
          (bind _output_get (set `self.Building` _returnvalue))
          ;[1 1 1] Trigger OnBuild
          (`Building.OnBuild` _output_get self))
        (:`then_1`
          ;[1 1 1] If claimed, tell Building about Settlement and Settlement about Building
          (`/Engine/EditorBlueprintResources/StandardMacros.IsValid` (`self.Claimant`)
            (:`Is Valid`
              (`Building.OnClaim` (`self.Building`) (`self.Claimant`))
              (`Settlement.OnBuildingAdded` (`self.Claimant`) (`self.Building`)))))
        (:`then_2`
          ;[1 1 1] Set Graphics
          (`StaticMeshComponent.SetStaticMesh` (`self.BuildingMesh`) (`BuildingDataAsset.Mesh` (`Building.DataAsset` (`self.Building`)))))
        (:`then_3`
          (`self.AddBuildingToReplication`)
          (return true))))))

(fn `Claim`
  (params (PotentialClaimant :type "Settlement Object Reference"))
  (returns (Success :type Boolean))
  ;[1 1 1] Can only be called by Server
  ;[1 1 1] not claimable
  (if (`self.IsClaimable`)
    (`|ExecutionSequence`
      (:`then_0`
        ;[1 1 1] Set instance variables
        (set `self.Claimant` (`local.PotentialClaimant`))
        (set `self.IsClaimable` false))
      (:`then_1`
        ;[1 0.452 0.332] Tell Building about Settlement and Settlement about Building
        (`/Engine/EditorBlueprintResources/StandardMacros.IsValid` (`self.Building`)
          (:`Is Valid`
            (`Building.OnClaim` (`self.Building`) (`self.Claimant`))
            (`Settlement.OnBuildingAdded` (`self.Claimant`) (`self.Building`)))))
      (:`then_2`
        (return true)))
    (else
      (return false))))

(fn `ClaimantChanged`
  (`/Engine/EditorBlueprintResources/StandardMacros.IsValid` (`self.Claimant`)
    (:`Is Valid`
      ;[1 1 1] Tile is now claimed
      (`SceneComponent.SetVisibility` (`self.ClaimMesh`) true false)
      (`MeshComponent.SetVectorParameterValueOnMaterials` (`self.ClaimMesh`) "Color" (`KismetMathLibrary.Conv_LinearColorToVector` (`Settlement.ClaimColor` (`self.Claimant`)))))
    (:`Is Not Valid`
      ;[1 1 1] Tile is not claimed anymore
      (`SceneComponent.SetVisibility` (`self.ClaimMesh`) false false))))

(fn `SpawnBuildingsOrProps`
  (params (SpawnPoints :type "Array of /Game/Core/World/Tile/F_SpawnPoint Structure") (MeshesToAdd :type "DataTable Object Reference"))
  (for _array_element SpawnPoints
    (bind _outrownames (`DataTableFunctionLibrary.GetDataTableRowNames` MeshesToAdd))
    (bind _returnvalue (`|GetDataTableRow` MeshesToAdd (`KismetArrayLibrary.Array_Random` _outrownames))
      (:`then`
        (bind _output_get (set `self.buildingRot` (`KismetMathLibrary.Conv_IntToDouble` (+ (`.DefaultZRotation_13_50A230644B179BE9100FA4BEB1EEA307` (break `/Game/Core/World/Tile/F_SpawnPoint` _array_element)) (* (`KismetMathLibrary.RandomIntegerInRange` 0 3) 90)))))
        (bind _returnvalue_2 (`AddComponent|NODE_AddStaticMeshComponent-6` :`RelativeTransform` (`KismetMathLibrary.MakeTransform` (break `/Game/Core/World/Tile/F_SpawnPoint` _array_element) (`KismetMathLibrary.MakeRotator` 0.0 0.0 _output_get))))
        (`ActorComponent.SetIsReplicated` _returnvalue_2 false)
        (bind (_staticmesh _skeletalmesh _animation) (break `/Game/Core/World/Tile/F_TileAsset` _returnvalue))
        (`StaticMeshComponent.SetStaticMesh` _returnvalue_2 _staticmesh)
        (bind _returnvalue_3 (`AddComponent|NODE_AddBP_GOTASkeletalMesh-4` :`RelativeTransform` (`KismetMathLibrary.MakeTransform` (break `/Game/Core/World/Tile/F_SpawnPoint` _array_element) (`KismetMathLibrary.MakeRotator` 0.0 0.0 _output_get))))
        (`ActorComponent.SetIsReplicated` _returnvalue_3 false)
        (`SkeletalMeshComponent.SetSkeletalMeshAsset` _returnvalue_3 _skeletalmesh)
        (`SkeletalMeshComponent.PlayAnimation` _returnvalue_3 _animation true)
        (`ActorComponent.SetComponentTickEnabled` _returnvalue_3 false)))))

(fn `Unbuild`
  ;[1 1 1] Can only be called by Server
  ;[1 1 1] Has no Building
  (`/Engine/EditorBlueprintResources/StandardMacros.IsValid` (`self.Building`)
    (:`Is Valid`
      (`|ExecutionSequence`
        (:`then_0`
          ;[1 1 1] If claimed, trigger OnUnclaim
          (`/Engine/EditorBlueprintResources/StandardMacros.IsValid` (`self.Claimant`)
            (:`Is Valid`
              (`Building.OnUnclaim` (`self.Building`) (`self.Claimant`))
              (`Settlement.OnBuildingRemoved` (`self.Claimant`) (`self.Building`)))))
        (:`then_1`
          ;[1 1 1] Trigger OnUnbuild of the Building
          (`Building.OnUnbuild` (`self.Building`) self))
        (:`then_2`
          ;[1 1 1] Set Graphics
          (`StaticMeshComponent.SetStaticMesh` (`self.BuildingMesh`) null))
        (:`then_3`
          ;[1 1 1] Remove Building reference
          (set `self.Building` null))))
    (:`Is Not Valid`
      (return))))

(fn `Unclaim`
  ;[1 1 1] Can only be called by Server
  ;[1 1 1] Has Claimant
  (`/Engine/EditorBlueprintResources/StandardMacros.IsValid` (`self.Claimant`)
    (:`Is Valid`
      (`|ExecutionSequence`
        (:`then_0`
          ;[1 0.452 0.332] Trigger Building Unclaim Effect if there is a Building on the Tile
          (`/Engine/EditorBlueprintResources/StandardMacros.IsValid` (`self.Building`)
            (:`Is Valid`
              (`Building.OnUnclaim` (`self.Building`) (`self.Claimant`))
              (`Settlement.OnBuildingRemoved` (`self.Claimant`) (`self.Building`)))))
        (:`then_1`
          ;[1 1 1] Tell Settlement that it lost this claim
          (`Settlement.LostClaim` (`self.Claimant`) self)
          (`Settlement.OnBuildingRemoved` (`self.Claimant`) (`self.Building`)))
        (:`then_2`
          ;[1 1 1] Set instance variables
          (set `self.Claimant` null)
          (set `self.IsClaimable` true))))
    (:`Is Not Valid`
      (return))))

(fn `UserConstructionScript`)