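; BP_TileContent manages the visual content of a world tile: trees, props and buildings.
; On a spawn layout change it rebuilds components at layout points, using random DataTable meshes for all trees and occasional props.
; Trees spawn hidden and get shuffled before UpdateTrees receives the tile's current count; buildings are placed as hidden placeholders, with no mesh assigned here.
; Animated meshes tick only while inside the player Guardian's active range.
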(event `self.OnEnteringActiveRangeOfGuardian`
  ;[1 0.8336 0.278] Activation / Deactivation of Animations when in range of the Player Guardian
  (set `self.IsActive` true)
  (for _array_element (`self.AnimatedMeshes`)
    (`ActorComponent.SetComponentTickEnabled` _array_element true)))

(event `self.OnLeavingActiveRangeOfGuardian`
  ;[1 0.8336 0.278] Activation / Deactivation of Animations when in range of the Player Guardian
  (set `self.IsActive` false)
  (for _array_element (`self.AnimatedMeshes`)
    (`ActorComponent.SetComponentTickEnabled` _array_element false)))

(event `self.OnSpawnPointLayoutChanged`
  (params (NewSpawnPointLayout :type "SpawnPointLayout Structure"))
  (bind (_locationontile _defaultrotation) (break `SpawnPoint` NewSpawnPointLayout_MainBuilding))
  (bind _mainbuilding (`self.MainBuilding`))
  ;[1 0.806 0.3364] Cleanup Old Trees
  (for _array_element (`self.TreeMeshes`)
    (`ActorComponent.K2_DestroyComponent` _array_element))
  (`KismetArrayLibrary.Array_Clear` (`self.TreeMeshes`))
  ;[1 0.8652 0.4328] Spawn All Trees and populate TreeMeshes
  (bind _outrownames (`DataTableFunctionLibrary.GetDataTableRowNames` (`self.TreeAssets`)))
  ;;[0.607 0.1344 1] loop
  (for _array_element_2 NewSpawnPointLayout_Trees
    (bind _returnvalue (`|GetDataTableRow` (`self.TreeAssets`) (`KismetArrayLibrary.Array_Random` _outrownames))
      (:`then`
        (bind _returnvalue_2 (`AddComponent|NODE_AddStaticMeshComponent-0`))
        (`StaticMeshComponent.SetStaticMesh` _returnvalue_2 (`.StaticMesh` (break `TileAsset` _returnvalue)))
        (`SceneComponent.K2_SetRelativeLocationAndRotation` _returnvalue_2 (`.LocationOnTile` (break `SpawnPoint` _array_element_2)) (`KismetMathLibrary.MakeRotator` 0.0 0.0 (`KismetMathLibrary.RandomFloatInRange` 0.0 359.0)) false true)
        (`SceneComponent.SetVisibility` _returnvalue_2 false false)
        (`KismetArrayLibrary.Array_Add` (`self.TreeMeshes`) _returnvalue_2))))
  ;[1 0.9734 0.2977] Set correct amount of Trees Visible
  (`KismetArrayLibrary.Array_Shuffle` (`self.TreeMeshes`))
  (`self.UpdateTrees` (`GOTAAttribute.Current` (`Tile.Trees` (`self.Tile`))))
  ;[1 0.806 0.3364] Cleanup Old Props
  (for _array_element_3 (`self.PropMeshes`)
    (`ActorComponent.K2_DestroyComponent` _array_element_3))
  (`KismetArrayLibrary.Array_Clear` (`self.PropMeshes`))
  ;[0.9716 1 0.427] Spawn New Props
  (for _array_element_4 NewSpawnPointLayout_Props
    (if (< (`KismetMathLibrary.RandomFloat`) 0.1)
      (bind _outrownames_2 (`DataTableFunctionLibrary.GetDataTableRowNames` (`self.PropAssets`)))
      (bind _returnvalue_3 (`|GetDataTableRow` (`self.PropAssets`) (`KismetArrayLibrary.Array_Random` _outrownames_2))
        (:`then`
          (bind _returnvalue_4 (`AddComponent|NODE_AddStaticMeshComponent-1`))
          (`StaticMeshComponent.SetStaticMesh` _returnvalue_4 (`.StaticMesh` (break `TileAsset` _returnvalue_3)))
          (`SceneComponent.K2_SetRelativeLocationAndRotation` _returnvalue_4 (`.LocationOnTile` (break `SpawnPoint` _array_element_4)) (`KismetMathLibrary.MakeRotator` 0.0 0.0 (`KismetMathLibrary.RandomFloatInRange` 0.0 359.0)) false true)
          (`KismetArrayLibrary.Array_Add` (`self.PropMeshes`) _returnvalue_4)))))
  ;[1 1 1] Set Position of Main Building
  (`SceneComponent.K2_SetRelativeLocationAndRotation` _mainbuilding _locationontile (`KismetMathLibrary.MakeRotator` 0.0 0.0 (`KismetMathLibrary.Conv_IntToDouble` _defaultrotation)) false true)
  (`SceneComponent.SetVisibility` _mainbuilding false false)
  ;[1 0.806 0.3364] Cleanup Old Props
  (for _array_element_5 (`self.BuildingMeshes`)
    (`ActorComponent.K2_DestroyComponent` _array_element_5))
  (`KismetArrayLibrary.Array_Clear` (`self.BuildingMeshes`))
  ;[1 1 1] Comment
  (for _array_element_6 NewSpawnPointLayout_Buildings
    (bind _returnvalue_5 (`AddComponent|NODE_AddStaticMeshComponent-2`))
    (bind (_locationontile_2 _defaultrotation_2) (break `SpawnPoint` _array_element_6))
    (`SceneComponent.K2_SetRelativeLocationAndRotation` _returnvalue_5 _locationontile_2 (`KismetMathLibrary.MakeRotator` 0.0 0.0 (`KismetMathLibrary.Conv_IntToDouble` _defaultrotation_2)) false true)
    (`SceneComponent.SetVisibility` _returnvalue_5 false false)
    (`KismetArrayLibrary.Array_Add` (`self.BuildingMeshes`) _returnvalue_5)))

(fn `UserConstructionScript`)