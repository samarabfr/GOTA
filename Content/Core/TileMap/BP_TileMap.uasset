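; BP_TileMap is the hex tile map that generates the world's tiles and answers tile queries.
; GenerateCircle loops over axial Q/R coordinates to build a hexagon of BP_Tile actors, offsetting height with randomly seeded FastNoise, and registers each by hex coordinate.
; Random tile, neighbor and path queries wrap Cpp-prefixed parent functions, casting their results to BP_Tile.
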(fn `ConvertToBPTileArray`
  (params (Tiles :type "Array of Tile Object Reference"))
  (returns (BP_Tiles :type "Array of /Game/Core/TileMap/BP_Tile Object Reference"))
  (locals (LOCAL_BP_Tiles :type "Array of /Game/Core/TileMap/BP_Tile Object Reference"))
  (for _array_element Tiles
    (bind _asbp_tile (cast `/Game/Core/TileMap/BP_Tile` _array_element))
    (`KismetArrayLibrary.Array_Add` (`local.LOCAL_BP_Tiles`) _asbp_tile))
  (return (`local.LOCAL_BP_Tiles`)))

(fn `GenerateCircle`
  (params (Radius :type Integer))
  (locals (Q :type Integer) (R :type Integer) (`Noise Wrapper` :type "FastNoiseWrapper Object Reference"))
  (bind _hexcoords (make `HexCoords` (`local.Q`) (`local.R`)))
  (bind (_x _y) (`KismetMathLibrary.BreakVector2D` (`self.HexCoordsToWorldPos` _hexcoords)))
  ;[1 1 1] Create Noise Wrapper
  (bind _returnvalue (`|GenericCreateObject` "/Script/FastNoiseGenerator.FastNoiseWrapper"))
  (bind _output_get (set `local.Noise Wrapper` _returnvalue))
  (`FastNoiseWrapper.SetupFastNoise` _output_get "Simplex" (`KismetMathLibrary.RandomInteger` 1000) 0.1 "Quintic" "FBM" 3 2.0 0.5 0.45 "Euclidean" "CellValue")
  ;[1 1 1] Q
  (for _index (range (* (`local.Radius`) -1) (+ (`local.Radius`) 1))
    (set `local.Q` _index)
    ;[1 1 1] R
    (for _index_2 (range (* (`local.Radius`) -1) (+ (`local.Radius`) 1))
      (set `local.R` _index_2)
      (if (<= (`KismetMathLibrary.Abs_Int` (+ (`local.Q`) (`local.R`))) (`local.Radius`))
        ;[1 1 1] I mean, we probably rework World generation anyways so it doesn't really matter how wank this is
        (`self.SpawnNewTile` (`KismetMathLibrary.MakeVector` _x _y (* (`FastNoiseWrapper.GetNoise2D` (`local.Noise Wrapper`) (/ _x (`self.HeightScale`)) (/ _y (`self.HeightScale`))) (`self.HeightScale`))) _hexcoords)))))

(fn `GetNeighboringTiles`
  (params (Tile :type "/Game/Core/TileMap/BP_Tile Object Reference"))
  (returns (NewParam :type "Array of /Game/Core/TileMap/BP_Tile Object Reference"))
  (locals (LOCALNeighbors :type "Array of /Game/Core/TileMap/BP_Tile Object Reference"))
  (return (`self.ConvertToBPTileArray` (`self.Cpp_GetNeighboringTiles` Tile))))

(fn `GetPath`
  (params (Start :type "/Game/Core/TileMap/BP_Tile Object Reference") (End :type "/Game/Core/TileMap/BP_Tile Object Reference"))
  (returns (Path :type "Array of /Game/Core/TileMap/BP_Tile Object Reference"))
  (locals (Frontier :type "Array of /Game/Core/TileMap/BP_Tile Object Reference") (CameFrom :type "Map of /Game/Core/TileMap/BP_Tile Object Reference to /Game/Core/TileMap/BP_Tile Object Reference") (Current :type "/Game/Core/TileMap/BP_Tile Object Reference") (Path :type "Array of /Game/Core/TileMap/BP_Tile Object Reference"))
  (return (`self.ConvertToBPTileArray` (`self.Cpp_GetPath` Start End))))

(fn `GetRandomTile`
  (returns (Tile :type "/Game/Core/TileMap/BP_Tile Object Reference"))
  (bind _asbp_tile (cast `/Game/Core/TileMap/BP_Tile` (`self.Cpp_GetRandomTile`)))
  (return _asbp_tile))

(fn `SpawnNewTile`
  (params (Location :type "Vector Structure") (Coords :type "HexCoords Structure"))
  (bind _returnvalue (`|SpawnActorFromClass` "/Game/Core/TileMap/BP_Tile.BP_Tile_C" (`KismetMathLibrary.MakeTransform` Location) "Undefined" "MultiplyWithRoot" self null))
  (`self.AddTile` Coords _returnvalue)
  (return))

(fn `UserConstructionScript`)