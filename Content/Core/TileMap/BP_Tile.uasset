(fn `Build`
  (params (`Building Class` :type "/Game/Core/BP_Building Class Reference"))
  (returns (Success :type Boolean))
  ;[1 1 1] Should only be called by Server
  ;[1 1 1] Already a Building on this Tile
  (`/Engine/EditorBlueprintResources/StandardMacros.IsValid` (`self.Building`)
    (:`Is Valid`
      (return false))
    (:`Is Not Valid`
      ;[1 1 1] Create Building Object
      (bind _returnvalue (`|GenericCreateObject` `Building Class`))
      (bind _output_get (set `self.Building` _returnvalue))
      ;[1 1 1] Trigger OnBuild
      (`/Game/Core/BP_Building.OnBuild` _output_get self)
      ;[1 1 1] If claimed, trigger OnClaim
      (`/Engine/EditorBlueprintResources/StandardMacros.IsValid` (`self.Claimant`)
        (:`Is Valid`
          (`/Game/Core/BP_Building.OnClaim` (`self.Building`) (`self.Claimant`))
          ;[1 1 1] Set Graphics
          (`StaticMeshComponent.SetStaticMesh` (`self.BuildingMesh`) (`/Game/Core/BP_BuildingDataAsset.Mesh` (`/Game/Core/BP_Building.DataAsset` (`self.Building`))))
          (return true))))))

(fn `Claim`
  (params (`Potential Claimant` :type "/Game/Core/BP_Settlement Object Reference"))
  (returns (Success :type Boolean))
  ;[1 1 1] Should only be called by Server
  ;[1 1 1] not claimable
  (if (`self.IsClaimable`)
    (`|ExecutionSequence`
      (:`then_0`
        ;[1 1 1] Set instance variables
        (set `self.Claimant` (`local.Potential Claimant`))
        (set `self.IsClaimable` false))
      (:`then_1`
        ;[1 0.452 0.332] Trigger Building Claim Effect if there is a Building on the Tile
        (`/Engine/EditorBlueprintResources/StandardMacros.IsValid` (`self.Building`)
          (:`Is Valid`
            (`/Game/Core/BP_Building.OnClaim` (`self.Building`) (`self.Claimant`)))))
      (:`then_2`
        (return true)))
    (else
      (return false))))

(fn `OnRep_Building`)

(fn `OnRep_Claimant`
  (`/Engine/EditorBlueprintResources/StandardMacros.IsValid` (`self.Claimant`)
    (:`Is Valid`
      ;[1 1 1] Tile is now claimed
      (`SceneComponent.SetVisibility` (`self.ClaimMesh`) true false)
      (`MeshComponent.SetVectorParameterValueOnMaterials` (`self.ClaimMesh`) "Color" (`KismetMathLibrary.Conv_LinearColorToVector` (`/Game/Core/BP_Settlement.ClaimColor` (`self.Claimant`)))))
    (:`Is Not Valid`
      ;[1 1 1] Tile is not claimed anymore
      (`SceneComponent.SetVisibility` (`self.ClaimMesh`) false false))))

(fn `OnRep_Height`)

(fn `OnRep_Nature`
  (`self.OnNatureChanged` (`self.Nature`)))

(fn `Unbuild`
  ;[1 1 1] Should only be called by Server
  ;[1 1 1] Has no Building
  (`/Engine/EditorBlueprintResources/StandardMacros.IsValid` (`self.Building`)
    (:`Is Valid`
      (`|ExecutionSequence`
        (:`then_0`
          ;[1 1 1] If claimed, trigger OnUnclaim
          (`/Engine/EditorBlueprintResources/StandardMacros.IsValid` (`self.Claimant`)
            (:`Is Valid`
              (`/Game/Core/BP_Building.OnUnclaim` (`self.Building`) (`self.Claimant`)))))
        (:`then_1`
          ;[1 1 1] Trigger OnUnbuild of the Building
          (`/Game/Core/BP_Building.OnUnbuild` (`self.Building`) self))
        (:`then_2`
          ;[1 1 1] Set Graphics
          (`StaticMeshComponent.SetStaticMesh` (`self.BuildingMesh`) null))
        (:`then_3`
          ;[1 1 1] Remove Building reference
          (set `self.Building` null))))
    (:`Is Not Valid`
      (return))))

(fn `Unclaim`
  ;[1 1 1] Should only be called by Server
  ;[1 1 1] Has Claimant
  (`/Engine/EditorBlueprintResources/StandardMacros.IsValid` (`self.Claimant`)
    (:`Is Valid`
      (`|ExecutionSequence`
        (:`then_0`
          ;[1 0.452 0.332] Trigger Building Unclaim Effect if there is a Building on the Tile
          (`/Engine/EditorBlueprintResources/StandardMacros.IsValid` (`self.Building`)
            (:`Is Valid`
              (`/Game/Core/BP_Building.OnUnclaim` (`self.Building`) (`self.Claimant`)))))
        (:`then_1`
          ;[1 1 1] Tell Settlement that it lost this claim
          (`/Game/Core/BP_Settlement.LostClaim` (`self.Claimant`) self))
        (:`then_2`
          ;[1 1 1] Set instance variables
          (set `self.Claimant` null)
          (set `self.IsClaimable` true))))
    (:`Is Not Valid`
      (return))))

(fn `UserConstructionScript`)