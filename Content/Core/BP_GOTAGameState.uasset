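; Game state that tracks a timed turn and map-wide totals of trees, forage and wildlife.
; Tick advances elapsed turn time up to a maximum unless paused, and NextTurn jumps it straight to that maximum.
; Registered tiles report resource changes through bound change events, which add each delta to the matching total, so totals update without polling.
; Turn rollover and timer reset are not handled in these graphs.
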(event `self.ReceiveTick`
  (params (DeltaSeconds :type "Float (single-precision)"))
  (if (`self.ShouldTickTurnTime`)
    (set `self.ElapsedTurnTime` (`KismetMathLibrary.FMin` (`self.MaxTurnTime`) (+ DeltaSeconds (`self.ElapsedTurnTime`))))))

(event `TogglePause`
  (set `self.ShouldTickTurnTime` (not (`self.ShouldTickTurnTime`))))

(event `self.RegisterTileForTotalsUpdates`
  (params (Tile :type "Tile Object Reference"))
  (add `GOTAAttribute.OnChanged` (`Tile.Trees` Tile) (delegate `UpdateTotalTrees`))
  (add `GOTAAttribute.OnChanged` (`Tile.Forage` Tile) (delegate `UpdateTotalForage`))
  (add `GOTAAttribute.OnChanged` (`Tile.Wildlife` Tile) (delegate `UpdateTotalWildlife`)))

(event `UpdateTotalTrees`
  (params (ChangedBy :type Integer))
  (`GOTAAttribute.Add` (`self.TotalTrees`) ChangedBy))

(event `UpdateTotalForage`
  (params (ChangedBy :type Integer))
  (`GOTAAttribute.Add` (`self.TotalForage`) ChangedBy))

(event `UpdateTotalWildlife`
  (params (ChangedBy :type Integer))
  (`GOTAAttribute.Add` (`self.TotalWildlife`) ChangedBy))

(fn `NextTurn`
  (set `self.ElapsedTurnTime` (`self.MaxTurnTime`)))

(fn `UserConstructionScript`)