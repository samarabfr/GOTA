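; BP_Guardian is the Guardian Blueprint, which receives a player controller and wires up that player's mouse utilities and abilities.
; SetPlayerController stores the controller, then spawns a BP_MouseUtils actor, noted as happening when a Guardian is created on the server, and makes the controller its owner.
; Both the controller and the mouse utilities are handed to BPGuardianAbilityManager, while the construction script is empty.
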(fn `SetPlayerController`
  (params (`Player Controller` :type "/Game/Core/BP_GOTAPlayerController Object Reference"))
  (set `self.PlayerController` `Player Controller`)
  ;[1 1 1] When a Guardian gets Created on Server it spawns its Mouse Utilities
  (bind _returnvalue (`|SpawnActorFromClass` "/Game/Core/BP_MouseUtils.BP_MouseUtils_C" (`KismetMathLibrary.MakeTransform` (0.0 0.0 0.0)) "Undefined" "MultiplyWithRoot" null null))
  (set `self.MouseUtils` _returnvalue)
  (set `/Game/Core/BP_MouseUtils.PlayerController` `Player Controller` (`self.MouseUtils`))
  (`self.SetOwner` (`self.MouseUtils`) `Player Controller`)
  (`/Game/Core/BP_GuardianAbilityManager.SetPlayerController` (`self.BP_GuardianAbilityManager`) `Player Controller`)
  (`/Game/Core/BP_GuardianAbilityManager.SetMouseUtils` (`self.BP_GuardianAbilityManager`) (`self.MouseUtils`)))

(fn `UserConstructionScript`)