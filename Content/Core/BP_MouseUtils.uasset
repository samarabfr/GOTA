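; BP_MouseUtils tracks a player's cursor position and hovered BP_Tile, sharing both across the network.
; Each tick the local controller traces under the cursor, moves the MousePosition component directly and passes the location to a networked variable.
; When the hovered tile changes, MouseTilePosition snaps to it and a HoverTileChanged dispatcher fires.
; OnRep functions move both components on receiving clients, and AttachToTilePosition lets actors follow the tile marker.
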(event `self.ReceiveTick`
  (params (DeltaSeconds :type "Float (single-precision)"))
  (bind (_bblockinghit _binitialoverlap _time _distance _location _impactpoint _normal _impactnormal _physmat _hitactor) (`GameplayStatics.BreakHitResult` (`PlayerController.GetHitResultUnderCursorByChannel` (`self.PlayerController`) "TraceTypeQuery1" true)))
  (`/Engine/EditorBlueprintResources/StandardMacros.IsValid` (`self.PlayerController`)
    (:`Is Valid`
      (if (`Controller.IsLocalController` (`self.PlayerController`))
        ;[1 1 1] Local Client Sets Location Directly and Sets Networked Position
        (`SceneComponent.K2_SetWorldLocation` (`self.MousePosition`) _location false false)
        (`self.SetNetworkedPosition` _location)
        ;[1 1 1] Local Client Checks for Hovering Tile Changed
        (bind _asbp_tile (cast `/Game/Core/TileMap/BP_Tile` _hitactor))
        (if (not (== (`self.HoverTile`) _asbp_tile))
          (set `self.HoverTile` _asbp_tile)
          (bind _returnvalue (`self.K2_GetActorLocation` _asbp_tile))
          (`SceneComponent.K2_SetWorldLocation` (`self.MouseTilePosition`) _returnvalue false false)
          (`self.SetNetworkedTilePosition` _returnvalue)
          (`self.HoverTileChanged` (`self.HoverTile`)))))))

(event `SetNetworkedPosition`
  (params (`New Position` :type "Vector Structure"))
  (set `self.NetworkedPosition` `New Position`))

(event `SetNetworkedTilePosition`
  (params (`New Tile Position` :type "Vector Structure"))
  (set `self.NetworkedTilePosition` `New Tile Position`))

(fn `AttachToTilePosition`
  (params (Actor :type "Actor Object Reference"))
  (`self.K2_AttachToComponent` Actor (`self.MouseTilePosition`) "None" "KeepRelative" "KeepRelative" "KeepRelative" true))

(fn `OnRep_NetworkedPosition`
  (`SceneComponent.K2_SetWorldLocation` (`self.MousePosition`) (`self.NetworkedPosition`) false false))

(fn `OnRep_NetworkedTilePosition`
  (`SceneComponent.K2_SetWorldLocation` (`self.MouseTilePosition`) (`self.NetworkedTilePosition`) false false))

(fn `UserConstructionScript`)