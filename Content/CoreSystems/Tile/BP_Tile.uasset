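; Hexagon map tile Blueprint that handles biome-based terrain visuals and relays Guardian range events.
; Entering or leaving the Guardian's active range is forwarded to TileContent, so animations can be disabled based on distance.
; The hexagon mesh takes its material from DATileGraphics by Biome, with grass getting random UV offsets to vary noise between tiles.
; ClaimantChanged is empty, as its claim visibility and color logic is disconnected.
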(event `self.OnEnteringActiveRangeOfGuardian`
  ;[1 0.826 0.3882] Activation Range for disabling Animations in a Range around the Guardian
  (`TileContent.OnEnteringActiveRangeOfGuardian` (`self.TileContent`)))

(event `self.OnLeavingActiveRangeOfGuardian`
  ;[1 0.826 0.3882] Activation Range for disabling Animations in a Range around the Guardian
  (`TileContent.OnLeavingActiveRangeOfGuardian` (`self.TileContent`)))

(event `self.UpdateHexagonMaterial`
  ;[1 0.2564 0.2066] Set Terrain Material dependend on Biome
  (switch `EBiome` (`self.Biome`)
    (:`Gras`
      (`PrimitiveComponent.SetMaterial` (`self.SM_Hexagon`) 0 (`TileGraphicsDataAsset.M_Grass` (`self.DA_TileGraphics`)))
      ;[1 0.3729 0.343] Set random offsets for material for noise variation between tiles
      (`MeshComponent.SetScalarParameterValueOnMaterials` (`self.SM_Hexagon`) "Offset U" (`KismetMathLibrary.RandomFloatInRange` 0.0 0.2))
      (`MeshComponent.SetScalarParameterValueOnMaterials` (`self.SM_Hexagon`) "Offset V" (`KismetMathLibrary.RandomFloatInRange` 0.0 0.2)))
    (:`Beach`
      (`PrimitiveComponent.SetMaterial` (`self.SM_Hexagon`) 0 (`TileGraphicsDataAsset.M_Beach` (`self.DA_TileGraphics`))))
    (:`Mountain`
      (`PrimitiveComponent.SetMaterial` (`self.SM_Hexagon`) 0 (`TileGraphicsDataAsset.M_Mountain` (`self.DA_TileGraphics`))))
    (:`Volcano`
      (`PrimitiveComponent.SetMaterial` (`self.SM_Hexagon`) 0 (`TileGraphicsDataAsset.M_Volcano` (`self.DA_TileGraphics`))))))

(fn `ClaimantChanged`)

(fn `UserConstructionScript`)