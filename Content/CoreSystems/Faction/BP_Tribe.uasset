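; BP_Tribe is a tribe faction Blueprint that handles the tribe's initial territory setup.
; InitialStartingSetup validates the given spawn tile, then claims it plus two random tiles, printing an error if the tile is invalid or unclaimable.
; A disconnected chain that would build on those tiles, seed population and culture followers, and stock starting food never runs.
; The construction script only calls its parent.
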(event `self.InitialStartingSetup`
  (params (SpawnTile :type "Tile Object Reference"))
  (`/Engine/EditorBlueprintResources/StandardMacros.IsValid` SpawnTile
    (:`Is Valid`
      (if (`Tile.IsClaimable` SpawnTile)
        (`self.ClaimTile` SpawnTile)
        (`self.ClaimRandomTile`)
        (`self.ClaimRandomTile`)
        (else
          (`KismetSystemLibrary.PrintString` "Settlement got invalid starting Tile" true true (struct :`G` 0.66 :`B` 1.0 :`A` 1.0) 10.0 :!label _label))))
    (:`Is Not Valid`
      (goto _label))))

(fn `UserConstructionScript`
  (`parent.UserConstructionScript`))