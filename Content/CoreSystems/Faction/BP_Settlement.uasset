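; Faction settlement actor that runs a turn-based economy, claims map tiles, constructs buildings and spawns armies.
; CalculateTurn adds production income and advances Expansion, which claims a tile at a threshold that scales with territory size.
; It holds one random new-building or tier-upgrade project until affordable, replacing it once built or impossible.
; Aggressive mood and overpopulation set the chance of spawning a BP_Army, which drains population from every building.
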(event `self.CalculateTurn`
  (`self.GenerateBaseIncome`)
  (`self.GenerateBuildingIncome`)
  (`self.FigureOutBuilding`)
  (`self.FigureOutSendingArmy`))

(event `self.GenerateBaseIncome`
  (bind _expansion (`self.Expansion`))
  (`|ExecutionSequence`
    (:`then_2`
      ;[1 1 1] Reached Expansion threshhold, base income +1
      (if (== (`GOTAAttribute.Current` _expansion) (`GOTAAttributeLimited.Maximum` _expansion))
        (`self.ClaimRandomTile`)
        (set `GOTAAttribute.Current` 1 (`self.Expansion`))
        (set `GOTAAttributeLimited.Maximum` (* 2 (`KismetArrayLibrary.Array_Length` (`self.ClaimedTiles`))) (`self.Expansion`))
        (else
          (`GOTAAttribute.Add` (`self.Expansion`) 1))))))

(event `self.GenerateBuildingIncome`
  (bind _value (`BlueprintMapLibrary.Map_Find` (`BuildingProductionSummary.ProductionMap` (`self.ProductionSummary`)) "Foraging"))
  (bind _returnvalue (/ _value 2))
  (`GOTAAttribute.Add` (`self.Food`) (- _value _returnvalue))
  (`GOTAAttribute.Add` (`self.Wood`) _returnvalue)
  (`GOTAAttribute.Add` (`self.Food`) (`BlueprintMapLibrary.Map_Find` (`BuildingProductionSummary.ProductionMap` (`self.ProductionSummary`)) "Hunting"))
  (`GOTAAttribute.Add` (`self.Wood`) (`BlueprintMapLibrary.Map_Find` (`BuildingProductionSummary.ProductionMap` (`self.ProductionSummary`)) "Woodcutting"))
  (`GOTAAttribute.Add` (`self.Expansion`) (`BlueprintMapLibrary.Map_Find` (`BuildingProductionSummary.ProductionMap` (`self.ProductionSummary`)) "Expansion")))

(event `self.FigureOutSendingArmy`
  ;[1 1 1] Minimum Pop to send out an Army
  (if (> (`PopulationSummary.Current` (`self.PopulationSummary`)) (`SettlementBalance.MinimumPopulationToSpawnArmy` (`self.SettlementBalance`)))
    ;[1 1 1] Calculate the Chance to send out an Army
    (bind _returnvalue (`PopulationSummary.GetMood` (`self.PopulationSummary`) "Aggressive"))
    (if (> (+ (* (/ (`KismetMathLibrary.Conv_IntToDouble` _returnvalue) (`KismetMathLibrary.Conv_IntToDouble` (`PopulationSummary.Current` (`self.PopulationSummary`)))) (`SettlementBalance.AggressiveMoodMaximumImpact` (`self.SettlementBalance`))) (* (`KismetMathLibrary.Conv_IntToDouble` (`KismetMathLibrary.Max` (- (`PopulationSummary.Current` (`self.PopulationSummary`)) (`SettlementBalance.HighPopulationThreshold` (`self.SettlementBalance`))))) (`SettlementBalance.HighPopulationImpact` (`self.SettlementBalance`)))) (`KismetMathLibrary.RandomFloat`))
      (bind _returnvalue_2 (`|SpawnActorFromClass` "/Game/CoreSystems/Entity/BP_Army.BP_Army_C" (`KismetMathLibrary.MakeTransform` (0.0 0.0 0.0)) "Undefined" "MultiplyWithRoot" null null))
      (`Entity.Init` _returnvalue_2 (`self.Affiliation`) (`KismetArrayLibrary.Array_Random` (`self.ClaimedTiles`)) 1)
      (for _array_element (`self.ClaimedTiles`)
        (bind _building (`Tile.Building` _array_element))
        (`/Engine/EditorBlueprintResources/StandardMacros.IsValid` _building
          (:`Is Valid`
            (`Population.ChangePopulation` (`Building.Population` _building) -2)))))))

(event `self.FigureOutBuilding`
  (`/Engine/EditorBlueprintResources/StandardMacros.IsValid` (`self.CurrentBuildingProject`)
    (:`Is Valid`
      (if (`BuildingProject.IsPossible` (`self.CurrentBuildingProject`))
        (if (`BuildingProject.CanAfford` (`self.CurrentBuildingProject`))
          (`BuildingProject.TryBuilding` (`self.CurrentBuildingProject`))
          (set `self.CurrentBuildingProject` null :!label _label)
          ;[1 1 1] Fill Building Pool with all possible building projects (new buildings or upgrades)
          (`KismetArrayLibrary.Array_Clear` (`self.BuildingProjectPool`) :!label _label_2)
          ;;[1 1 1] If there is a free building slot, add all possible Buildings to the pool
          (`KismetArrayLibrary.Array_Shuffle` (`self.ClaimedTiles`))
          (for _array_element (`self.ClaimedTiles`)
            (`/Engine/EditorBlueprintResources/StandardMacros.IsValid` (`Tile.Building` _array_element)
              (:`Is Not Valid`
                (for _array_element_2 (`self.PossibleBuildings`)
                  (bind _returnvalue (`|GenericCreateObject` "/Script/GOTA.BuildingProject"))
                  (`BuildingProject.Init` _returnvalue self _array_element_2 1 _array_element)
                  (`KismetArrayLibrary.Array_Add` (`self.BuildingProjectPool`) _returnvalue))
                (break))))
          (for _array_element_3 (`self.ClaimedTiles`)
            (bind _building (`Tile.Building` _array_element_3))
            (`/Engine/EditorBlueprintResources/StandardMacros.IsValid` _building
              (:`Is Valid`
                (bind _tier (`Building.Tier` _building))
                (bind _dataasset (`Building.DataAsset` _building))
                (if (and (== _tier 1) (> (`.Housing` (break `BuildingTierData` (`BuildingDataAsset.TierTwo` _dataasset))) 0))
                  (bind _returnvalue_2 (`|GenericCreateObject` "/Script/GOTA.BuildingProject"))
                  (`BuildingProject.Init` _returnvalue_2 self _dataasset 2 _array_element_3)
                  (`KismetArrayLibrary.Array_Add` (`self.BuildingProjectPool`) _returnvalue_2)
                  (elif (and (== _tier 2) (> (`.Housing` (break `BuildingTierData` (`BuildingDataAsset.TierThree` _dataasset))) 0))
                    (bind _returnvalue_3 (`|GenericCreateObject` "/Script/GOTA.BuildingProject"))
                    (`BuildingProject.Init` _returnvalue_3 self _dataasset 3 _array_element_3)
                    (`KismetArrayLibrary.Array_Add` (`self.BuildingProjectPool`) _returnvalue_3))))))
          ;[1 1 1] Select a Random Project. In future we should have some kind of logic to select which building project should be built
          (if (not (`KismetArrayLibrary.Array_IsEmpty` (`self.BuildingProjectPool`)))
            (set `self.CurrentBuildingProject` (`KismetArrayLibrary.Array_Random` (`self.BuildingProjectPool`)))))
        (else
          (goto _label))))
    (:`Is Not Valid`
      (goto _label_2))))

(fn `ClaimRandomNeighbor`
  (if (not (`BlueprintSetLibrary.Set_IsEmpty` (`self.BorderingUnclaimedTiles`)))
    (bind _result (`BlueprintSetLibrary.Set_ToArray` (`self.BorderingUnclaimedTiles`)))
    (`self.ClaimTile` (`KismetArrayLibrary.Array_Random` _result))))

(fn `ClaimTile`
  (params (Tile :type "Tile Object Reference"))
  (`/Engine/EditorBlueprintResources/StandardMacros.IsValid` Tile
    (:`Is Valid`
      (bind _returnvalue (`Tile.TryClaim` (`local.Tile`) self))
      (if _returnvalue
        (`KismetArrayLibrary.Array_Add` (`self.ClaimedTiles`) (`local.Tile`))
        (`self.RefreshBorderingTiles`)))))

(fn `LostClaim`
  (params (Tile :type "Tile Object Reference"))
  (`/Engine/EditorBlueprintResources/StandardMacros.IsValid` Tile
    (:`Is Valid`
      (`KismetArrayLibrary.Array_RemoveItem` (`self.ClaimedTiles`) (`local.Tile`))
      (`self.RefreshBorderingTiles`))))

(fn `RefreshBorderingTiles`
  (`BlueprintSetLibrary.Set_Clear` (`self.BorderingUnclaimedTiles`))
  (for _array_element (`self.ClaimedTiles`)
    (for _array_element_2 (`Tile.Neighbors` _array_element)
      (`/Engine/EditorBlueprintResources/StandardMacros.IsValid` _array_element_2
        (:`Is Valid`
          (if (`Tile.IsClaimable` _array_element_2)
            (`BlueprintSetLibrary.Set_Add` (`self.BorderingUnclaimedTiles`) _array_element_2)))))))

(fn `UserConstructionScript`)