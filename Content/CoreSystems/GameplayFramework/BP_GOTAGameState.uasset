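; BP_GOTAGameState is the game state that tracks turn timing and world-wide resource and population totals.
; Tick advances a capped, pausable turn timer, and NextTurn fills it to the maximum to end the turn early.
; Registered tiles feed tree, forage and wildlife totals through change bindings, while settlements register population summaries into colonial, native and overall totals.
; It also spawns and stores the static mesh batcher.
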(event `self.ReceiveTick`
  (params (DeltaSeconds :type "Float (single-precision)"))
  (if (`self.ShouldTickTurnTime`)
    (set `self.ElapsedTurnTime` (`KismetMathLibrary.FMin` (`self.MaxTurnTime`) (+ DeltaSeconds (`self.ElapsedTurnTime`))))))

(event `TogglePause`
  (set `self.ShouldTickTurnTime` (not (`self.ShouldTickTurnTime`))))

(event `self.SpawnStaticMeshBatcher`
  (bind _returnvalue (`|SpawnActorFromClass` "/Game/CoreSystems/Utility/BP_StaticMeshBatcher.BP_StaticMeshBatcher_C" (`KismetMathLibrary.MakeTransform` (0.0 0.0 0.0)) "Undefined" "MultiplyWithRoot" null null))
  (set `self.StaticMeshBatcher` _returnvalue))

(event `self.RegisterTileForTotalsUpdates`
  (params (Tile :type "Tile Object Reference"))
  (`GOTAAttribute.Add` (`self.TotalTrees`) (`GOTAAttribute.Current` (`Tile.Trees` Tile)))
  (add `GOTAAttribute.OnChanged` (`Tile.Trees` Tile) (delegate `UpdateTotalTrees`))
  (`GOTAAttribute.Add` (`self.TotalForage`) (`GOTAAttribute.Current` (`Tile.Forage` Tile)))
  (add `GOTAAttribute.OnChanged` (`Tile.Forage` Tile) (delegate `UpdateTotalForage`))
  (`GOTAAttribute.Add` (`self.TotalWildlife`) (`GOTAAttribute.Current` (`Tile.Wildlife` Tile)))
  (add `GOTAAttribute.OnChanged` (`Tile.Wildlife` Tile) (delegate `UpdateTotalWildlife`)))

(event `UpdateTotalTrees`
  (params (ChangedBy :type Integer))
  (`GOTAAttribute.Add` (`self.TotalTrees`) ChangedBy))

(event `UpdateTotalForage`
  (params (ChangedBy :type Integer))
  (`GOTAAttribute.Add` (`self.TotalForage`) ChangedBy))

(event `UpdateTotalWildlife`
  (params (ChangedBy :type Integer))
  (`GOTAAttribute.Add` (`self.TotalWildlife`) ChangedBy))

(event `self.RegisterColonialSettlementForTotalsUpdates`
  (params (Population :type "PopulationSummary Object Reference"))
  (`PopulationSummary.RegisterPopulationSummary` (`self.TotalColonialPopulation`) Population)
  (`PopulationSummary.RegisterPopulationSummary` (`self.TotalPopulation`) Population))

(event `self.RegisterNativeSettlementForTotalsUpdates`
  (params (Population :type "PopulationSummary Object Reference"))
  (`PopulationSummary.RegisterPopulationSummary` (`self.TotalNativePopulation`) Population)
  (`PopulationSummary.RegisterPopulationSummary` (`self.TotalPopulation`) Population))

(fn `NextTurn`
  (set `self.ElapsedTurnTime` (`self.MaxTurnTime`)))

(fn `UserConstructionScript`)