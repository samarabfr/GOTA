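; Loading manager that shows a loading screen and coordinates the multiplayer match startup between server and clients.
; The server spawns a loading status actor per player, then initializes game state and mode, creates map, factions and guardians, sets up player controllers and starts the game.
; Delay-based polling loops act as barriers on shared statuses.
; Clients follow the server's status and match its replication count before initializing UI and input.
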(event `self.InitLoadingScreen`
  (bind _returnvalue (`|CreateWidget` "/Game/UI/IngameUI/WBP_LoadingScreen.WBP_LoadingScreen_C" (`GameplayStatics.GetPlayerController` 0)))
  (bind _output_get (set `self.LoadingScreen` _returnvalue))
  (`UserWidget.AddToViewport` _output_get 0))

(event `self.RemoveLoadingScreen`
  (`Widget.SetVisibility` (`self.LoadingScreen`) "Hidden"))

(event `self.ReceiveBeginPlay`
  (`self.InitLoadingScreen`)
  (`/Engine/EditorBlueprintResources/ActorMacros.Switch Has Authority`
    (:`Authority`
      ;[1 0.2135 0.2135] Wait for All players to connect. Without the PlayerControllers nothing works ><
      (if (!= (`GOTAGameInstance.PlayerCount` (`/Game/CoreSystems/Utility/BPL_Utils.Get GOTA Game Instance`)) (`GameplayStatics.GetNumPlayerControllers`)) :!label _label
        (`KismetSystemLibrary.Delay` 0.5)
        (goto _label)
        (else
          ;[1 0.2552 0.2552] Init Loading Status Actors, they are responsible for sharing information about the loading process for every player
          (`self.Init`)
          (for _index (range (`GOTAGameInstance.PlayerCount` (`/Game/CoreSystems/Utility/BPL_Utils.Get GOTA Game Instance`)))
            (bind _returnvalue (`GameplayStatics.GetPlayerController` _index))
            (bind _returnvalue_2 (`|SpawnActorFromClass` "/Script/GOTA.LoadingStatusActor" (`KismetMathLibrary.MakeTransform` (0.0 0.0 0.0)) "Undefined" "MultiplyWithRoot" _returnvalue null))
            (`self.K2_AttachToActor` _returnvalue_2 _returnvalue "None" "KeepRelative" "KeepRelative" "KeepRelative" true)
            (`self.SetOwner` _returnvalue_2 _returnvalue)
            (set `LoadingStatusActor.GOTAPlayerID` _index _returnvalue_2)
            (`KismetArrayLibrary.Array_Set` (`self.LoadingStatuses`) _index _returnvalue_2))
          (set `self.LoadingStatus` (`|GetArrayItem` (`self.LoadingStatuses`)))
          ;[1 0.2552 0.2552] Server Loading Process
          (`LoadingStatusActor.SetCurrentStatus` (`self.LoadingStatus`) "WaitForAllPlayersReadyToStartLoading")
          (`/Game/UI/IngameUI/WBP_LoadingScreen.InitLoadingBars` (`self.LoadingScreen`) (`self.LoadingStatuses`))
          (set `self.ReadyCheck` true :!label _label_2)
          (for _array_element (`self.LoadingStatuses`)
            (if (not (`|EnumEquality` (`LoadingStatusActor.CurrentStatus` _array_element) "WaitForAllPlayersReadyToStartLoading"))
              (set `self.ReadyCheck` false)))
          (if (`self.ReadyCheck`)
            (`LoadingStatusActor.SetCurrentStatus` (`self.LoadingStatus`) "InitializingGameState")
            (bind _output_get (set `self.GameState` (`/Game/CoreSystems/Utility/BPL_Utils.Get GOTA Game State`)))
            (`GS_Ingame.Init` _output_get)
            (set `GS_Ingame.LoadingManager` self (`self.GameState`))
            (bind _asbp_gm_ingame (cast `/Game/CoreSystems/GameplayFramework/BP_GM_Ingame` (`GameplayStatics.GetGameMode`))
              (:`then`
                (bind _output_get_2 (set `self.GameMode` _asbp_gm_ingame))
                (`GM_Ingame.Init` _output_get_2)
                (`LoadingStatusActor.SetCurrentStatus` (`self.LoadingStatus`) "WaitForAllPlayersReadyForCreation")
                (set `self.ReadyCheck` true :!label _label_3)
                (for _array_element_2 (`self.LoadingStatuses`)
                  (if (not (`|EnumEquality` (`LoadingStatusActor.CurrentStatus` _array_element_2) "WaitForAllPlayersReadyForCreation"))
                    (set `self.ReadyCheck` false)))
                (if (`self.ReadyCheck`)
                  (`LoadingStatusActor.SetCurrentStatus` (`self.LoadingStatus`) "CreateMap")
                  (`GM_Ingame.CreateMap` (`self.GameMode`))
                  (`LoadingStatusActor.SetCurrentStatus` (`self.LoadingStatus`) "CreateFactions")
                  (`GM_Ingame.CreateFactions` (`self.GameMode`))
                  (`LoadingStatusActor.SetCurrentStatus` (`self.LoadingStatus`) "CreateGuardians")
                  (`GM_Ingame.CreateGuardians` (`self.GameMode`))
                  (`LoadingStatusActor.SetCurrentStatus` (`self.LoadingStatus`) "WaitingForAllPlayersReplication")
                  (`LoadingStatusActor.SetNetworkedReplicationCount` (`self.LoadingStatus`) (`LoadingStatusActor.ReplicationCount` (`self.LoadingStatus`)))
                  (set `self.ReadyCheck` true :!label _label_4)
                  (for _array_element_3 (`self.LoadingStatuses`)
                    (if (not (`|EnumEquality` (`LoadingStatusActor.CurrentStatus` _array_element_3) "WaitingForAllPlayersReplication"))
                      (set `self.ReadyCheck` false)))
                  (if (`self.ReadyCheck`)
                    (`LoadingStatusActor.SetCurrentStatus` (`self.LoadingStatus`) "InitPlayerControllers")
                    (for _index_2 (range (`GameplayStatics.GetNumPlayerControllers`))
                      (bind _asbp_pc_ingame (cast `/Game/CoreSystems/GameplayFramework/BP_PC_Ingame` (`GameplayStatics.GetPlayerController` _index_2))
                        (:`then`
                          (`PC_Ingame.Init` _asbp_pc_ingame))
                        (:`CastFailed`
                          (`KismetSystemLibrary.PrintString` "Using the wrong Player Controller"))))
                    (`LoadingStatusActor.SetCurrentStatus` (`self.LoadingStatus`) "PlayerControllerPossession")
                    (`GM_Ingame.InitialPlayerControllerPossession` (`self.GameMode`))
                    (`LoadingStatusActor.SetCurrentStatus` (`self.LoadingStatus`) "InitializingUI")
                    (bind _asbp_pc_ingame_2 (cast `/Game/CoreSystems/GameplayFramework/BP_PC_Ingame` (`GameplayStatics.GetPlayerController` 0))
                      (:`then`
                        (`PC_Ingame.InitUI` _asbp_pc_ingame_2)
                        (`LoadingStatusActor.SetCurrentStatus` (`self.LoadingStatus`) "Finished")
                        (bind _aspc_ingame (cast `PC_Ingame` (`GameplayStatics.GetPlayerController` 0)))
                        (`PC_Ingame.InitInput` _aspc_ingame)
                        (`KismetSystemLibrary.Delay` 0.2)
                        (`self.RemoveLoadingScreen`)
                        (`KismetSystemLibrary.Delay` 0.2)
                        (`GM_Ingame.StartGame` (`self.GameMode`)))
                      (:`CastFailed`
                        (`KismetSystemLibrary.PrintString` "Using Wrong PlayerController. Should use BP_GOTAPlayerController" true true (struct :`G` 0.66 :`B` 1.0 :`A` 1.0) 200.0)))
                    (else
                      (`KismetSystemLibrary.Delay` 1.0)
                      (goto _label_4)))
                  (else
                    (`KismetSystemLibrary.Delay` 1.0)
                    (goto _label_3))))
              (:`CastFailed`
                (`KismetSystemLibrary.PrintString` "Using Wrong Gamemode. Should use BP_GOTAGameMode" true true (struct :`G` 0.66 :`B` 1.0 :`A` 1.0) 200.0)))
            (else
              (`KismetSystemLibrary.Delay` 1.0)
              (goto _label_2))))))
    (:`Remote`
      ;[0.2656 1 0.2656] Client Loading Process
      ;;[1 1 1] Wait for Replication of GOTAPlayerState and GOTAPlayerID, the Server is always 0 so clients now they got their correct ID when they aren't 0
      (bind _asps_ingame (cast `PS_Ingame` (`Controller.PlayerState` (`GameplayStatics.GetPlayerController` 0)) :!label _label_5)
        (:`then`
          (bind _gotaplayerid (`PS_Ingame.GOTAPlayerID` _asps_ingame))
          (if (== 0 _gotaplayerid)
            (`KismetSystemLibrary.Delay` 1.0 :!label _label_6)
            (goto _label_5)
            (else
              (set `self.GOTAPlayerID` _gotaplayerid)
              ;;[1 1 1] Wait for LoadingStatus to replicate
              (`/Engine/EditorBlueprintResources/StandardMacros.IsValid` (`|GetArrayItem` (`self.LoadingStatuses`) (`self.GOTAPlayerID`)) :!label _label_7
                (:`Is Valid`
                  (set `self.LoadingStatus` (`|GetArrayItem` (`self.LoadingStatuses`) (`self.GOTAPlayerID`)))
                  (`LoadingStatusActor.SetCurrentStatus` (`self.LoadingStatus`) "WaitForAllPlayersReadyToStartLoading")
                  (`/Game/UI/IngameUI/WBP_LoadingScreen.InitLoadingBars` (`self.LoadingScreen`) (`self.LoadingStatuses`))
                  ;;[1 1 1] Wait until Server is done initializing Core
                  (if (`|EnumEquality` (`LoadingStatusActor.CurrentStatus` (`|GetArrayItem` (`self.LoadingStatuses`))) "WaitForAllPlayersReadyForCreation") :!label _label_8
                    (bind _output_get_3 (set `self.GameState` (`/Game/CoreSystems/Utility/BPL_Utils.Get GOTA Game State`)))
                    (set `GS_Ingame.LoadingManager` self (`self.GameState`))
                    (bind _returnvalue_3 (`|SpawnActorFromClass` "/Game/CoreSystems/Utility/BP_StaticMeshBatcher.BP_StaticMeshBatcher_C" (`KismetMathLibrary.MakeTransform` (0.0 0.0 0.0)) "Undefined" "MultiplyWithRoot" null null))
                    (set `GS_Ingame.StaticMeshBatcher` _returnvalue_3 _output_get_3)
                    (`LoadingStatusActor.SetCurrentStatus` (`self.LoadingStatus`) "WaitForAllPlayersReadyForCreation")
                    ;;[1 1 1] Wait until Server started Creating
                    (if (> (`KismetSystemLibrary.MakeLiteralByte` (`LoadingStatusActor.CurrentStatus` (`|GetArrayItem` (`self.LoadingStatuses`)))) (`KismetSystemLibrary.MakeLiteralByte` (enumliteral `ELoadingStatus` "WaitForAllPlayersReadyForCreation"))) :!label _label_9
                      (`LoadingStatusActor.SetCurrentStatus` (`self.LoadingStatus`) "Replicating")
                      ;;[1 1 1] Wait for the server to finish creating and client finish replicating
                      (`LoadingStatusActor.SetNetworkedReplicationCount` (`self.LoadingStatus`) (`LoadingStatusActor.ReplicationCount` (`self.LoadingStatus`)) :!label _label_10)
                      (if (and (== (`LoadingStatusActor.NetworkedReplicationCount` (`self.LoadingStatus`)) (`LoadingStatusActor.NetworkedReplicationCount` (`|GetArrayItem` (`self.LoadingStatuses`)))) (`|EnumEquality` (`LoadingStatusActor.CurrentStatus` (`|GetArrayItem` (`self.LoadingStatuses`))) "WaitingForAllPlayersReplication") (!= (`LoadingStatusActor.NetworkedReplicationCount` (`|GetArrayItem` (`self.LoadingStatuses`))) 0))
                        (`LoadingStatusActor.SetCurrentStatus` (`self.LoadingStatus`) "WaitingForAllPlayersReplication")
                        ;;[1 1 1] Wait for the Server to finish Loading
                        (if (`|EnumEquality` (`LoadingStatusActor.CurrentStatus` (`|GetArrayItem` (`self.LoadingStatuses`))) "Finished") :!label _label_11
                          (bind _aspc_ingame_2 (cast `PC_Ingame` (`GameplayStatics.GetPlayerController` 0)))
                          (`PC_Ingame.InitUI` _aspc_ingame_2)
                          (`KismetSystemLibrary.Delay` 0.2)
                          (`PC_Ingame.InitInput` _aspc_ingame_2)
                          (`KismetSystemLibrary.Delay` 0.2)
                          (`self.RemoveLoadingScreen`)
                          (else
                            (`KismetSystemLibrary.Delay` 0.5)
                            (goto _label_11)))
                        (else
                          (`KismetSystemLibrary.Delay` 1.0)
                          (goto _label_10)))
                      (else
                        (`KismetSystemLibrary.Delay` 0.5)
                        (goto _label_9)))
                    (else
                      (`KismetSystemLibrary.Delay` 0.5)
                      (goto _label_8))))
                (:`Is Not Valid`
                  (`KismetSystemLibrary.Delay` 1.0)
                  (goto _label_7))))))
        (:`CastFailed`
          (goto _label_6))))))

(fn `UserConstructionScript`)