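; In-game GameMode that sets up a match and runs its timed turn loop on the server.
; Setup events spawn the tile map, colonist and native settlements, and the selected guardians, then have each player controller possess a guardian.
; Authority-only Tick runs a synchronous turn calculation when the GameState turn timer expires, pausing the timer and printing the duration.
; Each turn resolves settlements, combat, entity movement, then the tile map.
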(event `self.ReceiveTick`
  (params (DeltaSeconds :type "Float (single-precision)"))
  (`/Engine/EditorBlueprintResources/ActorMacros.Switch Has Authority`
    (:`Authority`
      (`/Engine/EditorBlueprintResources/StandardMacros.IsValid` (`self.Game State`)
        (:`Is Valid`
          (if (`GS_Ingame.ShouldTickTurnTime` (`self.Game State`))
            ;[1 1 1] Check if Turn is finished
            (if (>= (`/Game/CoreSystems/GameplayFramework/BP_GS_Ingame.ElapsedTurnTime` (`self.Game State`)) (`/Game/CoreSystems/GameplayFramework/BP_GS_Ingame.MaxTurnTime` (`self.Game State`)))
              (`GS_Ingame.MulticastSetElapsedTurnTime` (`self.Game State`) 0.0)
              (`self.NotAsyncTurnCalc`))))))))

(event `NotAsyncTurnCalc`
  (`self.OnTurnCalculationStart`)
  (`self.CalculateTurn`)
  (`self.OnTurnCalculationEnd`))

(event `OnTurnCalculationStart`
  (set `GS_Ingame.ShouldTickTurnTime` false (`self.Game State`))
  (set `GS_Ingame.IsCalculatingTurn` true (`self.Game State`))
  (set `self.TurnCalculationTime` (`KismetMathLibrary.Now`))
  (`GS_Ingame.CallCalculationStart` (`self.Game State`)))

(event `OnTurnCalculationEnd`
  (bind (_days _hours _minutes _seconds _fractionnano) (`KismetMathLibrary.BreakTimespan2` (- (`KismetMathLibrary.Now`) (`self.TurnCalculationTime`))))
  (set `GS_Ingame.ShouldTickTurnTime` true (`self.Game State`))
  (set `GS_Ingame.IsCalculatingTurn` false (`self.Game State`))
  (`KismetSystemLibrary.PrintString` (`KismetStringLibrary.Concat_StrStr` "Turn calc time (ms): " (`KismetStringLibrary.Conv_IntToString` (+ (* _seconds 1000) (/ _fractionnano 1000000)))))
  (`GS_Ingame.CallCalculationEnd` (`self.Game State`)))

(event `self.Init`
  ;[1 1 1] Game State
  (set `self.Game State` (`/Game/CoreSystems/Utility/BPL_Utils.Get GOTA Game State`)))

(event `self.CreateMap`
  ;[1 1 1] creating the TileMap
  (bind _returnvalue (`|SpawnActorFromClass` "/Game/CoreSystems/Tile/BP_TileMap.BP_TileMap_C" (`KismetMathLibrary.MakeTransform` (0.0 0.0 0.0)) "Undefined" "MultiplyWithRoot" null null))
  (bind _output_get (set `GS_Ingame.TileMap` _returnvalue (`self.Game State`)))
  (`TileMap.GenerateTiles` _output_get 600))

(event `self.CreateFactions`
  ;[0.3542 0.3542 0.3542] Factions
  ;;[1 1 1] Colonists
  (for _ (range (+ (`GOTAGameInstance.ColonistsSettlementCount` (`/Game/CoreSystems/Utility/BPL_Utils.Get GOTA Game Instance`)) 1))
    (bind _returnvalue (`|SpawnActorFromClass` "/Game/Factions/Colonists/BP_Colony.BP_Colony_C" (`KismetMathLibrary.MakeTransform` (0.0 0.0 0.0)) "Undefined" "MultiplyWithRoot" null null))
    (`Settlement.Init` _returnvalue)
    (set `Settlement.Affiliation` "Enemy" _returnvalue)
    (`KismetArrayLibrary.Array_Add` (`GS_Ingame.ColonistsSettlements` (`self.Game State`)) _returnvalue))
  ;;[1 1 1] Natives
  (for _ (range (+ (`GOTAGameInstance.NativesSettlementCount` (`/Game/CoreSystems/Utility/BPL_Utils.Get GOTA Game Instance`)) 1))
    (bind _returnvalue_2 (`|SpawnActorFromClass` "/Game/Factions/Natives/BP_Tribe.BP_Tribe_C" (`KismetMathLibrary.MakeTransform` (0.0 0.0 0.0)) "Undefined" "MultiplyWithRoot" null null))
    (`Settlement.Init` _returnvalue_2)
    (set `Settlement.Affiliation` "Ally" _returnvalue_2)
    (`KismetArrayLibrary.Array_Add` (`GS_Ingame.NativeSettlements` (`self.Game State`)) _returnvalue_2)))

(event `self.CreateGuardians`
  (bind _selectedguardian1 (`GOTAGameInstance.SelectedGuardian1` (`/Game/CoreSystems/Utility/BPL_Utils.Get GOTA Game Instance`)))
  (bind _selectedguardian2 (`GOTAGameInstance.SelectedGuardian2` (`/Game/CoreSystems/Utility/BPL_Utils.Get GOTA Game Instance`)))
  (bind _selectedguardian3 (`GOTAGameInstance.SelectedGuardian3` (`/Game/CoreSystems/Utility/BPL_Utils.Get GOTA Game Instance`)))
  (bind _selectedguardian4 (`GOTAGameInstance.SelectedGuardian4` (`/Game/CoreSystems/Utility/BPL_Utils.Get GOTA Game Instance`)))
  (`|ExecutionSequence`
    (:`then_0`
      (if (`KismetSystemLibrary.IsValidClass` _selectedguardian1)
        (bind _returnvalue (`|SpawnActorFromClass` _selectedguardian1 (`KismetMathLibrary.MakeTransform` (0.0 0.0 1000.0)) "AdjustIfPossibleButAlwaysSpawn" "MultiplyWithRoot" null null))
        (`KismetArrayLibrary.Array_Add` (`GS_Ingame.Guardians` (`self.Game State`)) _returnvalue)))
    (:`then_1`
      (if (`KismetSystemLibrary.IsValidClass` _selectedguardian2)
        (bind _returnvalue_2 (`|SpawnActorFromClass` _selectedguardian2 (`KismetMathLibrary.MakeTransform` (0.0 0.0 1000.0)) "AdjustIfPossibleButAlwaysSpawn" "MultiplyWithRoot" null null))
        (`KismetArrayLibrary.Array_Add` (`GS_Ingame.Guardians` (`self.Game State`)) _returnvalue_2)))
    (:`then_2`
      (if (`KismetSystemLibrary.IsValidClass` _selectedguardian3)
        (bind _returnvalue_3 (`|SpawnActorFromClass` _selectedguardian3 (`KismetMathLibrary.MakeTransform` (0.0 0.0 1000.0)) "AdjustIfPossibleButAlwaysSpawn" "MultiplyWithRoot" null null))
        (`KismetArrayLibrary.Array_Add` (`GS_Ingame.Guardians` (`self.Game State`)) _returnvalue_3)))
    (:`then_3`
      (if (`KismetSystemLibrary.IsValidClass` _selectedguardian4)
        (bind _returnvalue_4 (`|SpawnActorFromClass` _selectedguardian4 (`KismetMathLibrary.MakeTransform` (0.0 0.0 1000.0)) "AdjustIfPossibleButAlwaysSpawn" "MultiplyWithRoot" null null))
        (`KismetArrayLibrary.Array_Add` (`GS_Ingame.Guardians` (`self.Game State`)) _returnvalue_4)))))

(event `self.InitialPlayerControllerPossession`
  (for _index (range (`GameplayStatics.GetNumPlayerControllers`))
    (bind _asbp_pc_ingame (cast `/Game/CoreSystems/GameplayFramework/BP_PC_Ingame` (`GameplayStatics.GetPlayerController` _index))
      (:`then`
        (bind _asbp_guardian (cast `/Game/CoreSystems/Guardian/BP_Guardian` (`|GetArrayItem` (`GS_Ingame.Guardians` (`self.Game State`)) _index)))
        (`/Game/CoreSystems/GameplayFramework/BP_PC_Ingame.Possess Guardian` _asbp_pc_ingame _asbp_guardian))
      (:`CastFailed`
        (`KismetSystemLibrary.PrintString` "Using the wrong Player Controller")))))

(event `self.StartGame`
  (set `GS_Ingame.ShouldTickTurnTime` true (`self.Game State`)))

(fn `CalculateTurn`
  (`|ExecutionSequence`
    (:`then_1`
      ;[1 1 1] Settlements Turns
      (for _array_element (`GS_Ingame.ColonistsSettlements` (`self.Game State`))
        (`/Game/CoreSystems/Faction/BP_Settlement.CalculateTurn` _array_element))
      (for _array_element_2 (`GS_Ingame.NativeSettlements` (`self.Game State`))
        (`/Game/CoreSystems/Faction/BP_Settlement.CalculateTurn` _array_element_2)))
    (:`then_2`
      ;[1 1 1] Combat Phase
      (for _array_element_3 (`GS_Ingame.TileEntities` (`self.Game State`))
        (if (`Entity.ShouldCombatTrigger` _array_element_3)
          (`Entity.TriggerCombat` _array_element_3))))
    (:`then_3`
      ;[1 1 1] Tile Entities Movement
      (for _array_element_4 (`GS_Ingame.TileEntities` (`self.Game State`))
        (`Entity.CalculateMovement` _array_element_4)))
    (:`then_4`
      ;[1 1 1] Nature berechnen
      (`TileMap.CalculateTurn` (`GS_Ingame.TileMap` (`self.Game State`))))))

(fn `UserConstructionScript`)